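; Camera-view snap puzzle where the player drags physics pieces over highlighted holes in a tiled background.
; The construction script builds the grid, picks a random hole layout from a data table and spawns the pieces.
; A looping timer drives cursor dragging, while opposite-tagged socket boxes snap pieces together with spawned, locked physics constraints.
; Touching a bar resets the pieces; matching hole overlap count to layout size makes them glow and disables the bars.
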(event `/Game/CPCP2/Utilities/Character/Blueprints/BP_PuzzleInterface.DeactivateCamera`
  ;[1 1 1] Exit Puzzle
  (`KismetSystemLibrary.K2_ClearAndInvalidateTimerHandle` (`self.TimerHandle`))
  (for _array_element (`self.Snappables`)
    (bind _asstatic_mesh_component (cast `StaticMeshComponent` _array_element))
    (`PrimitiveComponent.SetRenderCustomDepth` _asstatic_mesh_component false)))

(event `/Game/CPCP2/Utilities/Character/Blueprints/BP_PuzzleInterface.ActivateCamera`
  (bind _returnvalue (`GameplayStatics.GetPlayerController` 0))
  (bind (_returnvalue_x _returnvalue_y) (`KismetMathLibrary.BreakVector2D` (`WidgetLayoutLibrary.GetViewportSize`)))
  (bind _returnvalue_2 (`GameplayStatics.GetPlayerController` 0))
  (bind _returnvalue_3 (`GameplayStatics.GetPlayerController` 0))
  ;[1 1 1] Enter To Puzzle
  (`PlayerController.SetMouseLocation` _returnvalue_2 (`KismetMathLibrary.FTrunc` (/ _returnvalue_x 2.0)) (`KismetMathLibrary.FTrunc` (/ _returnvalue_y 2.0)))
  (`WidgetBlueprintLibrary.SetInputMode_GameAndUIEx` _returnvalue_2 null "DoNotLock" false)
  (`Controller.SetIgnoreLookInput` _returnvalue_3 true)
  (`Controller.SetIgnoreMoveInput` _returnvalue_3 true)
  (`PlayerController.SetViewTargetWithBlend` _returnvalue_3 self 0.5 "VTBlend_Linear" 0.0 false)
  (set `PlayerController.bEnableClickEvents` true _returnvalue)
  (set `PlayerController.bEnableMouseOverEvents` true _returnvalue)
  (set `PlayerController.bShowMouseCursor` true _returnvalue)
  (`WidgetLayoutLibrary.RemoveAllWidgets`)
  ;[1 1 1] Drag And Drop
  (bind _returnvalue_4 (`KismetSystemLibrary.K2_SetTimerDelegate` (delegate `TimerEvent`) (`GameplayStatics.GetWorldDeltaSeconds`) true))
  (set `self.TimerHandle` _returnvalue_4))

(event `TimerEvent`
  (bind _returnvalue (`GameplayStatics.GetPlayerController` 0))
  (bind (_worldlocation _worlddirection) (`PlayerController.DeprojectMousePositionToWorld` (`GameplayStatics.GetPlayerController` 0)))
  (bind _hitresult (`PlayerController.GetHitResultUnderCursorForObjects` (`GameplayStatics.GetPlayerController` 0) (`|MakeArray` "ObjectTypeQuery4" :!type "EObjectTypeQuery Enum") true))
  (bind (_returnvalue_x _returnvalue_y _returnvalue_z) (`KismetMathLibrary.BreakVector` (`KismetMathLibrary.InverseTransformLocation` (`KismetMathLibrary.Conv_VectorToTransform` (`self.RelativeGrabLocation`)) (+ _worldlocation (* _worlddirection (`.Distance` (`GameplayStatics.BreakHitResult` _hitresult)))))))
  ;[1 1 1] Drag And Drop
  (bind _asbp_puzzle_character (cast `/Game/CPCP2/Utilities/Character/Blueprints/BP_PuzzleCharacter` (`GameplayStatics.GetPlayerCharacter` 0)))
  (if (or (not (`self.IsOnReleased`)) (`/Game/CPCP2/Utilities/Character/Blueprints/BP_PuzzleCharacter.isPuzzleActive` _asbp_puzzle_character))
    (if (`GameplayStatics.BreakHitResult` _hitresult)
      (for _array_element (`self.Snappables`)
        (bind _asstatic_mesh_component (cast `StaticMeshComponent` _array_element))
        (if (== _asstatic_mesh_component (`.HitComponent` (`GameplayStatics.BreakHitResult` _hitresult)))
          (`PrimitiveComponent.SetRenderCustomDepth` _asstatic_mesh_component true)
          (set `PlayerController.CurrentMouseCursor` "GrabHand" _returnvalue)
          (for _array_element_2 (`self.Snappables`)
            (bind _asstatic_mesh_component_2 (cast `StaticMeshComponent` _array_element_2))
            (if (!= _asstatic_mesh_component_2 _asstatic_mesh_component)
              (`PrimitiveComponent.SetRenderCustomDepth` _asstatic_mesh_component_2 false)
              (if (`self.IsOnClicked`)
                (set `PlayerController.CurrentMouseCursor` "GrabHandClosed" _returnvalue)
                (bind _returnvalue_x_2 (`KismetMathLibrary.BreakVector` (`SceneComponent.K2_GetComponentLocation` _asstatic_mesh_component)))
                (`SceneComponent.K2_SetWorldLocation` _asstatic_mesh_component (`KismetMathLibrary.MakeVector` _returnvalue_x_2 _returnvalue_y _returnvalue_z) false false))))))
      (else
        (for _array_element_3 (`self.Snappables`) :!label _label
          (bind _asstatic_mesh_component_3 (cast `StaticMeshComponent` _array_element_3))
          (`PrimitiveComponent.SetRenderCustomDepth` _asstatic_mesh_component_3 false)
          (set `PlayerController.CurrentMouseCursor` "Default" _returnvalue))))
    (else
      (goto _label))))

(event `self.ReceiveActorOnClicked`
  (params (ButtonPressed :type "Key Structure"))
  (bind _hitresult (`PlayerController.GetHitResultUnderCursorForObjects` (`GameplayStatics.GetPlayerController` 0) (`|MakeArray` "ObjectTypeQuery4" :!type "EObjectTypeQuery Enum") true))
  ;[1 1 1] Click And Release
  (set `self.IsOnClicked` true)
  (set `self.IsOnReleased` false)
  (bind _asbp_puzzle_character (cast `/Game/CPCP2/Utilities/Character/Blueprints/BP_PuzzleCharacter` (`GameplayStatics.GetPlayerCharacter` 0)))
  (if (or (not (`self.IsOnReleased`)) (`/Game/CPCP2/Utilities/Character/Blueprints/BP_PuzzleCharacter.isPuzzleActive` _asbp_puzzle_character))
    (if (`GameplayStatics.BreakHitResult` _hitresult)
      (for _array_element (`self.Snappables`)
        (bind _asstatic_mesh_component (cast `StaticMeshComponent` _array_element))
        (if (== _asstatic_mesh_component (`.HitComponent` (`GameplayStatics.BreakHitResult` _hitresult)))
          (set `self.ClickedComponent` _asstatic_mesh_component)
          (set `self.RelativeGrabLocation` (`KismetMathLibrary.InverseTransformLocation` (`KismetMathLibrary.Conv_VectorToTransform` (`SceneComponent.K2_GetComponentLocation` _asstatic_mesh_component)) (`.Location` (`GameplayStatics.BreakHitResult` _hitresult)))))))))

(event `self.ReceiveActorOnReleased`
  (params (ButtonReleased :type "Key Structure"))
  ;[1 1 1] Click And Release
  (set `self.IsOnClicked` false)
  (set `self.IsOnReleased` true)
  (for _array_element (`self.Snappables`)
    (bind _asstatic_mesh_component (cast `StaticMeshComponent` _array_element))
    (`PrimitiveComponent.SetRenderCustomDepth` _asstatic_mesh_component false)))

(event `self.Bar1.OnComponentBeginOverlap`
  (params (OverlappedComponent :type "PrimitiveComponent Object Reference") (OtherActor :type "Actor Object Reference") (OtherComp :type "PrimitiveComponent Object Reference") (OtherBodyIndex :type Integer) (bFromSweep :type Boolean) (SweepResult :type "HitResult Structure (by ref)"))
  ;[1 1 1] Lose Condition
  (`|ExecutionSequence` :!label _label_2
    (:`then_0`
      (set `self.IsOnClicked` false)
      (set `self.IsOnReleased` true)
      (for _array_element (`self.Snappables`)
        (bind _asstatic_mesh_component (cast `StaticMeshComponent` _array_element))
        (`PrimitiveComponent.SetRenderCustomDepth` _asstatic_mesh_component false)))
    (:`then_1`
      (bind _outactors (`GameplayStatics.GetAllActorsOfClass` "/Script/Engine.PhysicsConstraintActor"))
      (for _array_element_2 _outactors
        (`self.K2_DestroyActor` _array_element_2)))
    (:`then_2`
      (for (_array_element_3 _array_index) (`self.Snappables`)
        (`PrimitiveComponent.SetSimulatePhysics` _array_element_3 false)
        (`SceneComponent.K2_SetWorldTransform` _array_element_3 (`|GetArrayItem` (`self.SnappablesOriginalTransforms`) _array_index) false false)))
    (:`then_3`
      (for _array_element_4 (`self.Snappables`)
        (`PrimitiveComponent.SetSimulatePhysics` _array_element_4 true)))
    (:`then_4`
      (for _array_element_5 (`self.BoxCollisions`)
        (`PrimitiveComponent.SetCollisionEnabled` _array_element_5 "QueryOnly")))))

(event `self.Bar2.OnComponentBeginOverlap`
  (params (OverlappedComponent :type "PrimitiveComponent Object Reference") (OtherActor :type "Actor Object Reference") (OtherComp :type "PrimitiveComponent Object Reference") (OtherBodyIndex :type Integer) (bFromSweep :type Boolean) (SweepResult :type "HitResult Structure (by ref)"))
  ;[1 1 1] Lose Condition
  (goto _label_2))

(event `self.Bar3.OnComponentBeginOverlap`
  (params (OverlappedComponent :type "PrimitiveComponent Object Reference") (OtherActor :type "Actor Object Reference") (OtherComp :type "PrimitiveComponent Object Reference") (OtherBodyIndex :type Integer) (bFromSweep :type Boolean) (SweepResult :type "HitResult Structure (by ref)"))
  ;[1 1 1] Lose Condition
  (goto _label_2))

(event `self.Bar4.OnComponentBeginOverlap`
  (params (OverlappedComponent :type "PrimitiveComponent Object Reference") (OtherActor :type "Actor Object Reference") (OtherComp :type "PrimitiveComponent Object Reference") (OtherBodyIndex :type Integer) (bFromSweep :type Boolean) (SweepResult :type "HitResult Structure (by ref)"))
  ;[1 1 1] Lose Condition
  (goto _label_2))

(event `self.ReceiveTick`
  (params (DeltaSeconds :type "Float (single-precision)"))
  ;[1 1 1] Win Condition
  (if (== (`KismetArrayLibrary.Array_Length` (`self.WinArray`)) (`KismetArrayLibrary.Array_Length` (`self.WinBools`)))
    (for _array_element (`self.Snappables`)
      (`MeshComponent.SetScalarParameterValueOnMaterials` _array_element "Intensity" 10.0)
      (`PrimitiveComponent.SetCollisionEnabled` (`self.Bar2`) "NoCollision")
      (`PrimitiveComponent.SetCollisionEnabled` (`self.Bar3`) "NoCollision")
      (`PrimitiveComponent.SetCollisionEnabled` (`self.Bar4`) "NoCollision")
      (`PrimitiveComponent.SetCollisionEnabled` (`self.Bar1`) "NoCollision"))))

(fn `BackgroundOnOverlapBegin`
  (params (OverlappedComponent :type "PrimitiveComponent Object Reference") (OtherActor :type "Actor Object Reference") (OtherComp :type "PrimitiveComponent Object Reference") (OtherBodyIndex :type Integer) (bFromSweep :type Boolean) (SweepResult :type "HitResult Structure (by ref)"))
  ;[1 1 1] Overlap Begin
  (bind _asmesh_component (cast `MeshComponent` (`SceneComponent.GetAttachParent` OverlappedComponent)))
  (`MeshComponent.SetVectorParameterValueOnMaterials` _asmesh_component "Roll" (`KismetMathLibrary.Conv_LinearColorToVector` (struct :`G` 0.226713 :`B` 1.0 :`A` 1.0)))
  (`KismetArrayLibrary.Array_Add` (`self.WinBools`) true))

(fn `BackgroundOnOverlapEnd`
  (params (OverlappedComponent :type "PrimitiveComponent Object Reference") (OtherActor :type "Actor Object Reference") (OtherComp :type "PrimitiveComponent Object Reference") (OtherBodyIndex :type Integer))
  (bind _winbools (`self.WinBools`))
  ;[1 1 1] Overlap End
  (bind _asmesh_component (cast `MeshComponent` (`SceneComponent.GetAttachParent` OverlappedComponent)))
  (`MeshComponent.SetVectorParameterValueOnMaterials` _asmesh_component "Roll" (0.0 0.0 0.0))
  (if (> (`KismetArrayLibrary.Array_Length` _winbools) 0)
    (`KismetArrayLibrary.Array_Remove` _winbools)))

(fn `SnapOnOverlapBegin`
  (params (OverlappedComponent :type "PrimitiveComponent Object Reference") (OtherActor :type "Actor Object Reference") (OtherComp :type "PrimitiveComponent Object Reference") (OtherBodyIndex :type Integer) (bFromSweep :type Boolean) (SweepResult :type "HitResult Structure (by ref)"))
  (bind _returnvalue (`SceneComponent.GetAttachParent` OverlappedComponent))
  (bind _returnvalue_location (`KismetMathLibrary.BreakTransform` (`SceneComponent.K2_GetComponentToWorld` _returnvalue)))
  ;[1 1 1] On Overlap Begin
  (bind _output_get (set `self.Overlapped Component` OverlappedComponent))
  (bind _output_get_2 (set `self.Other Comp` OtherComp))
  (bind _output (`|GetArrayItem` (`ActorComponent.ComponentTags` _output_get)))
  (set `self.OverlapCompnentTag` _output)
  (bind _componenttags (`ActorComponent.ComponentTags` _output_get_2))
  (if (> (`KismetArrayLibrary.Array_Length` _componenttags) 0)
    (bind _output_2 (`|GetArrayItem` _componenttags))
    (set `self.OtherComponentTag` _output_2)
    (if (and (!= (`self.OverlapCompnentTag`) (`self.OtherComponentTag`)) (or (and (== (`self.OtherComponentTag`) "Right") (== (`self.OverlapCompnentTag`) "Left")) (and (== (`self.OtherComponentTag`) "Left") (== (`self.OverlapCompnentTag`) "Right")) (and (== (`self.OtherComponentTag`) "Up") (== (`self.OverlapCompnentTag`) "Down")) (and (== (`self.OtherComponentTag`) "Down") (== (`self.OverlapCompnentTag`) "Up")) (and (== (`self.OtherComponentTag`) "Front") (== (`self.OverlapCompnentTag`) "Back")) (and (== (`self.OtherComponentTag`) "Back") (== (`self.OverlapCompnentTag`) "Front"))))
      (bind _returnvalue_location_2 (`KismetMathLibrary.BreakTransform` (`SceneComponent.GetSocketTransform` OtherComp _output_2 "RTS_World")))
      (bind _returnvalue_location_3 (`KismetMathLibrary.BreakTransform` (`SceneComponent.GetSocketTransform` OverlappedComponent _output "RTS_World")))
      (`SceneComponent.K2_SetWorldLocation` _returnvalue (+ _returnvalue_location (/ (- _returnvalue_location_2 _returnvalue_location_3) 1)) false false)
      (`|ExecutionSequence`
        (:`then_0`
          (bind _asstatic_mesh_component (cast `StaticMeshComponent` (`SceneComponent.GetAttachParent` OverlappedComponent)))
          (bind _asstatic_mesh_component_2 (cast `StaticMeshComponent` (`SceneComponent.GetAttachParent` OtherComp))))
        (:`then_1`
          (bind _outactors (`GameplayStatics.GetAllActorsOfClass` "/Script/Engine.PhysicsConstraintActor"))
          (for _array_element _outactors
            (bind (_outcomponent1 _outbonename1 _outcomponent2) (`PhysicsConstraintComponent.GetConstrainedComponents` (`PhysicsConstraintActor.ConstraintComp` _array_element)))))
        (:`then_2`
          (if (and (!= _outcomponent2 _asstatic_mesh_component) (!= _outcomponent1 _asstatic_mesh_component_2))
            (bind _returnvalue_2 (`|SpawnActorFromClass` "/Script/Engine.PhysicsConstraintActor" (`SceneComponent.K2_GetComponentToWorld` _returnvalue) "Undefined" "OverrideRootScale" null null))
            (bind _constraintcomp (`PhysicsConstraintActor.ConstraintComp` _returnvalue_2))
            (bind _returnvalue_3 (`PhysicsConstraintComponent.GetConstraint` _constraintcomp))
            (`ConstraintInstanceBlueprintLibrary.SetDisableCollision` _returnvalue_3 true)
            (`ConstraintInstanceBlueprintLibrary.SetLinearLimits` _returnvalue_3 "LCM_Locked" "LCM_Locked" "LCM_Locked")
            (`ConstraintInstanceBlueprintLibrary.SetAngularLimits` _returnvalue_3 "ACM_Locked" 0.0 "ACM_Locked" 0.0 "ACM_Locked")
            (`ConstraintInstanceBlueprintLibrary.SetAngularDriveParams` _returnvalue_3)
            (`ConstraintInstanceBlueprintLibrary.SetProjectionParams` _returnvalue_3 true)
            (bind _asstatic_mesh_component_3 (cast `StaticMeshComponent` (`SceneComponent.GetAttachParent` OverlappedComponent)))
            (bind _asstatic_mesh_component_4 (cast `StaticMeshComponent` (`SceneComponent.GetAttachParent` OtherComp)))
            (`PhysicsConstraintComponent.SetConstrainedComponents` _constraintcomp _asstatic_mesh_component_3 "None" _asstatic_mesh_component_4 "None")
            (bind _asbox_collision (cast `BoxComponent` OverlappedComponent))
            (`PrimitiveComponent.SetCollisionEnabled` _asbox_collision "NoCollision")
            (bind _asbox_collision_2 (cast `BoxComponent` OtherComp))
            (`PrimitiveComponent.SetCollisionEnabled` _asbox_collision_2 "NoCollision")))))))

(fn `UserConstructionScript`
  (bind _tilesize (`self.TileSize`))
  (bind _backgroundmax (`self.BackgroundMax`))
  (bind _backgroundtilesize (`self.BackgroundTileSize`))
  (bind _returnvalue (/ (* _backgroundtilesize _backgroundmax) 2.0))
  (bind _returnvalue_2 (`KismetMathLibrary.FTrunc` (`KismetMathLibrary.Sqrt` (`KismetMathLibrary.Conv_IntToDouble` (`self.DescriptionLength`)))))
  (bind _returnvalue_3 (/ (* _tilesize _returnvalue_2) 2.0))
  (`|ExecutionSequence`
    (:`then_0`
      ;[1 1 1] Set Camera Transform
      (`SceneComponent.K2_SetRelativeTransform` (`self.Camera`) (`self.CameraTransform`) false false))
    (:`then_1`
      ;[1 1 1] Tiles
      (for _index (range (* _backgroundmax _backgroundmax))
        (bind _returnvalue_4 (`AddComponent|NODE_AddStaticMeshComponent-7` :`RelativeTransform` (`KismetMathLibrary.MakeTransform` (`KismetMathLibrary.MakeVector` -48.0 (- (`KismetMathLibrary.Conv_IntToDouble` (* (mod _index _backgroundmax) _backgroundtilesize)) _returnvalue) (- (`KismetMathLibrary.Conv_IntToDouble` (* (/ _index _backgroundmax) _backgroundtilesize)) _returnvalue)) (struct :`Roll` 90.0) (`self.BackgroundTileVectorSize`))))
        (`KismetArrayLibrary.Array_AddUnique` (`self.BackgroundTiles`) _returnvalue_4)
        (bind _returnvalue_5 (`AddComponent|NODE_AddTextRenderComponent-0`))
        (`TextRenderComponent.K2_SetText` _returnvalue_5 (`KismetTextLibrary.Conv_IntToText` _index))
        (`SceneComponent.K2_AttachToComponent` _returnvalue_5 _returnvalue_4 "Text" "KeepRelative" "KeepRelative" "KeepRelative" true)
        (`SceneComponent.SetVisibility` _returnvalue_5 (`self.IsEditMode`) false)
        (`SceneComponent.SetVisibility` _returnvalue_4 true false)))
    (:`then_2`
      ;[1 1 1] Generate holes from data table and bind overlap events
      (if (not (`self.IsEditMode`))
        (bind _returnvalue_6 (`|GetDataTableRow` "/Game/CPCP2/Snap/Blueprints/DT_SnapDescriptionDataTable.DT_SnapDescriptionDataTable" (`KismetStringLibrary.Conv_StringToName` (`KismetStringLibrary.Conv_IntToString` (`KismetMathLibrary.RandomInteger` 3))))
          (:`then`
            (set `self.DescriptionLength` (`KismetArrayLibrary.Array_Length` (break `/Game/CPCP2/Snap/Blueprints/F_SnapDescriptionStruct` _returnvalue_6)))
            (bind _output_get (set `self.WinArray` (break `/Game/CPCP2/Snap/Blueprints/F_SnapDescriptionStruct` _returnvalue_6)))
            (for _array_element _output_get
              (bind _output (`|GetArrayItem` (`self.BackgroundTiles`) _array_element))
              (`MeshComponent.SetVectorParameterValueOnMaterials` _output "Roll" (0.0 0.0 0.0))
              (bind _returnvalue_7 (`AddComponent|NODE_AddBoxComponent-3` :`RelativeTransform` (`KismetMathLibrary.MakeTransform` (-50.0 0.0 0.0))))
              (`SceneComponent.K2_AttachToComponent` _returnvalue_7 _output "Back" "KeepRelative" "KeepRelative" "KeepRelative" true)
              (add `PrimitiveComponent.OnComponentEndOverlap` _returnvalue_7 (`|CreateDelegate` :!event `BackgroundOnOverlapEnd`))
              (add `PrimitiveComponent.OnComponentBeginOverlap` _returnvalue_7 (`|CreateDelegate` :!event `BackgroundOnOverlapBegin`)))))))
    (:`then_4`
      ;[1 1 1] Snap Manager
      (for _index_2 (range (* _returnvalue_2 _returnvalue_2))
        ;;[0.9093 1 0] Simulate Physics On
        (bind _returnvalue_8 (`AddComponent|NODE_AddStaticMeshComponent-0` :`RelativeTransform` (`KismetMathLibrary.MakeTransform` (`KismetMathLibrary.MakeVector` -60.0 (+ (- (`KismetMathLibrary.Conv_IntToDouble` (* (mod _index_2 _returnvalue_2) _tilesize)) _returnvalue_3) 2.5) (+ (- (`KismetMathLibrary.Conv_IntToDouble` (* (/ _index_2 _returnvalue_2) _tilesize)) _returnvalue_3) 2.5)) (struct) (0.2 0.2 0.2))))
        (`KismetArrayLibrary.Array_AddUnique` (`self.Snappables`) _returnvalue_8)
        (`KismetArrayLibrary.Array_AddUnique` (`self.SnappablesOriginalTransforms`) (`SceneComponent.K2_GetComponentToWorld` _returnvalue_8))
        (`SceneComponent.SetVisibility` _returnvalue_8 (not (`self.IsEditMode`)) false)))
    (:`then_5`
      (for _array_element_2 (`self.Snappables`)
        (if (`ActorComponent.ComponentHasTag` _array_element_2 "Snappable")
          (for _array_element_3 (`SceneComponent.GetAllSocketNames` _array_element_2)
            (bind (_returnvalue_location _returnvalue_rotation _returnvalue_scale) (`KismetMathLibrary.BreakTransform` (`SceneComponent.GetSocketTransform` _array_element_2 _array_element_3 "RTS_World")))
            (bind _returnvalue_9 (`AddComponent|NODE_AddBoxComponent-0` :`RelativeTransform` (`KismetMathLibrary.MakeTransform` _returnvalue_location _returnvalue_rotation (/ _returnvalue_scale 1))))
            (set `ActorComponent.ComponentTags` (`|MakeArray` _array_element_3) _returnvalue_9)
            (`SceneComponent.K2_AttachToComponent` _returnvalue_9 _array_element_2 _array_element_3 "SnapToTarget" "SnapToTarget" "KeepRelative" true)
            (add `PrimitiveComponent.OnComponentBeginOverlap` _returnvalue_9 (`|CreateDelegate` :!event `SnapOnOverlapBegin`))
            (`KismetArrayLibrary.Array_AddUnique` (`self.BoxCollisions`) _returnvalue_9)))))))