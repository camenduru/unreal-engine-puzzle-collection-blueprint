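; BP_InventoryPuzzle is a puzzle actor where the player drags pieces over a generated tile grid in a dedicated camera view.
; Activation blends to the view, enables the cursor and shows the inventory widget if unsolved; exiting clears unsolved pieces.
; A looping timer traces under the cursor to drag Cube's child meshes in Y/Z.
; Nine children count as a win regardless of position, raising their material Intensity.
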(event `/Game/CPCP2/Utilities/Character/Blueprints/BP_PuzzleInterface.DeactivateCamera`
  ;[1 1 1] Exit Puzzle
  (`KismetSystemLibrary.K2_ClearAndInvalidateTimerHandle` (`self.TimerHandle`))
  (if (not (`self.IsWin`))
    (bind _output_get (set `self.Pieces` (`SceneComponent.GetChildrenComponents` (`self.Cube`) true)))
    (for _array_element _output_get
      (`ActorComponent.K2_DestroyComponent` _array_element))))

(event `/Game/CPCP2/Utilities/Character/Blueprints/BP_PuzzleInterface.ActivateCamera`
  (bind (_returnvalue_x _returnvalue_y) (`KismetMathLibrary.BreakVector2D` (`WidgetLayoutLibrary.GetViewportSize`)))
  (bind _returnvalue (`GameplayStatics.GetPlayerController` 0))
  (bind _returnvalue_2 (`GameplayStatics.GetPlayerController` 0))
  (bind _returnvalue_3 (`GameplayStatics.GetPlayerController` 0))
  ;[1 1 1] Enter To Puzzle
  (`PlayerController.SetMouseLocation` _returnvalue_3 (`KismetMathLibrary.FTrunc` (/ _returnvalue_x 2.0)) (`KismetMathLibrary.FTrunc` (/ _returnvalue_y 2.0)))
  (`WidgetBlueprintLibrary.SetInputMode_GameAndUIEx` _returnvalue_3 null "DoNotLock" false)
  (`Controller.SetIgnoreLookInput` _returnvalue true)
  (`Controller.SetIgnoreMoveInput` _returnvalue true)
  (`PlayerController.SetViewTargetWithBlend` _returnvalue self 0.5 "VTBlend_Linear" 0.0 false)
  (set `PlayerController.bEnableClickEvents` true _returnvalue_2)
  (set `PlayerController.bEnableMouseOverEvents` true _returnvalue_2)
  (set `PlayerController.bShowMouseCursor` true _returnvalue_2)
  (`WidgetLayoutLibrary.RemoveAllWidgets`)
  ;[1 1 1] Drag And Drop
  (bind _returnvalue_4 (`KismetSystemLibrary.K2_SetTimerDelegate` (delegate `TimerEvent`) (`self.TickTime`) true))
  (set `self.TimerHandle` _returnvalue_4)
  (if (not (`self.IsWin`))
    (bind _returnvalue_5 (`|CreateWidget` "/Game/CPCP2/Inventory/Blueprints/WBP_InventoryWidget.WBP_InventoryWidget_C"))
    (`UserWidget.AddToViewport` _returnvalue_5 0)))

(event `TimerEvent`
  (bind _returnvalue (`GameplayStatics.GetPlayerController` 0))
  (bind (_worldlocation _worlddirection) (`PlayerController.DeprojectMousePositionToWorld` (`GameplayStatics.GetPlayerController` 0)))
  (bind _children (`SceneComponent.GetChildrenComponents` (`self.Cube`) true))
  (bind _hitresult (`PlayerController.GetHitResultUnderCursorForObjects` (`GameplayStatics.GetPlayerController` 0) (`|MakeArray` "ObjectTypeQuery7" :!type "EObjectTypeQuery Enum") true))
  (bind (_returnvalue_x _returnvalue_y _returnvalue_z) (`KismetMathLibrary.BreakVector` (`KismetMathLibrary.InverseTransformLocation` (`KismetMathLibrary.Conv_VectorToTransform` (`self.RelativeGrabLocation`)) (+ _worldlocation (* _worlddirection (`.Distance` (`GameplayStatics.BreakHitResult` _hitresult)))))))
  ;[1 1 1] Drag And Drop
  (`|ExecutionSequence`
    (:`then_0`
      (bind _asbp_puzzle_character (cast `/Game/CPCP2/Utilities/Character/Blueprints/BP_PuzzleCharacter` (`GameplayStatics.GetPlayerCharacter` 0)))
      (if (or (not (`self.IsOnReleased`)) (`/Game/CPCP2/Utilities/Character/Blueprints/BP_PuzzleCharacter.isPuzzleActive` _asbp_puzzle_character))
        (if (`GameplayStatics.BreakHitResult` _hitresult)
          (for _array_element (`SceneComponent.GetChildrenComponents` (`self.Cube`) true)
            (bind _asstatic_mesh_component (cast `StaticMeshComponent` _array_element))
            (if (== _asstatic_mesh_component (`.HitComponent` (`GameplayStatics.BreakHitResult` _hitresult)))
              (`PrimitiveComponent.SetRenderCustomDepth` _asstatic_mesh_component false)
              (set `PlayerController.CurrentMouseCursor` "GrabHand" _returnvalue)
              (for _array_element_2 (`SceneComponent.GetChildrenComponents` (`self.Cube`) true)
                (bind _asstatic_mesh_component_2 (cast `StaticMeshComponent` _array_element_2))
                (if (!= _asstatic_mesh_component_2 _asstatic_mesh_component)
                  (`PrimitiveComponent.SetRenderCustomDepth` _asstatic_mesh_component_2 false)
                  (if (`self.IsOnClicked`)
                    (set `PlayerController.CurrentMouseCursor` "GrabHandClosed" _returnvalue)
                    (bind _returnvalue_x_2 (`KismetMathLibrary.BreakVector` (`SceneComponent.K2_GetComponentLocation` _asstatic_mesh_component)))
                    (`SceneComponent.K2_SetWorldLocation` _asstatic_mesh_component (`KismetMathLibrary.MakeVector` _returnvalue_x_2 _returnvalue_y _returnvalue_z) false false))))))
          (else
            (for _array_element_3 (`SceneComponent.GetChildrenComponents` (`self.Cube`) true) :!label _label
              (bind _asstatic_mesh_component_3 (cast `StaticMeshComponent` _array_element_3))
              (`PrimitiveComponent.SetRenderCustomDepth` _asstatic_mesh_component_3 false)
              (set `PlayerController.CurrentMouseCursor` "Default" _returnvalue))))
        (else
          (goto _label))))
    (:`then_1`
      ;[1 1 1] Win Condition
      (if (== (`KismetArrayLibrary.Array_Length` _children) 9)
        (for _array_element_4 _children
          (bind _asstatic_mesh_component_4 (cast `StaticMeshComponent` _array_element_4))
          (`MeshComponent.SetScalarParameterValueOnMaterials` _asstatic_mesh_component_4 "Intensity" 200.0)
          (set `self.IsWin` true))))))

(event `self.ReceiveActorOnClicked`
  (params (ButtonPressed :type "Key Structure"))
  (bind _hitresult (`PlayerController.GetHitResultUnderCursorForObjects` (`GameplayStatics.GetPlayerController` 0) (`|MakeArray` "ObjectTypeQuery7" :!type "EObjectTypeQuery Enum") true))
  ;[1 1 1] Click And Release
  (set `self.IsOnClicked` true)
  (set `self.IsOnReleased` false)
  (bind _asbp_puzzle_character (cast `/Game/CPCP2/Utilities/Character/Blueprints/BP_PuzzleCharacter` (`GameplayStatics.GetPlayerCharacter` 0)))
  (if (or (not (`self.IsOnReleased`)) (`/Game/CPCP2/Utilities/Character/Blueprints/BP_PuzzleCharacter.isPuzzleActive` _asbp_puzzle_character))
    (if (`GameplayStatics.BreakHitResult` _hitresult)
      (for _array_element (`SceneComponent.GetChildrenComponents` (`self.Cube`) true)
        (bind _asstatic_mesh_component (cast `StaticMeshComponent` _array_element))
        (if (== _asstatic_mesh_component (`.HitComponent` (`GameplayStatics.BreakHitResult` _hitresult)))
          (set `self.ClickedComponent` _asstatic_mesh_component)
          (set `self.RelativeGrabLocation` (`KismetMathLibrary.InverseTransformLocation` (`KismetMathLibrary.Conv_VectorToTransform` (`SceneComponent.K2_GetComponentLocation` _asstatic_mesh_component)) (`.Location` (`GameplayStatics.BreakHitResult` _hitresult)))))))))

(event `self.ReceiveActorOnReleased`
  (params (ButtonReleased :type "Key Structure"))
  ;[1 1 1] Click And Release
  (set `self.IsOnClicked` false)
  (set `self.IsOnReleased` true))

(event `InputAction|LeftMouseButton`
  (params (Key :type "Key Structure"))
  ;[1 1 1] Click And Release
  (:`Pressed`
    (set `self.IsOnClicked` false)
    (set `self.IsOnReleased` true)))

(fn `UserConstructionScript`
  (bind _tilesize (`self.TileSize`))
  (bind _max (`self.Max`))
  (`|ExecutionSequence`
    (:`then_0`
      ;[1 1 1] Init Generate Tiles
      (for _index (range (* _max _max))
        (bind _returnvalue (`AddComponent|NODE_AddStaticMeshComponent-0` :`RelativeTransform` (`KismetMathLibrary.MakeTransform` (`KismetMathLibrary.MakeVector` 0.0 (`KismetMathLibrary.Conv_IntToDouble` (- (* (mod _index _max) _tilesize) 76)) (`KismetMathLibrary.Conv_IntToDouble` (- (* (/ _index _max) _tilesize) 76))) (struct :`Yaw` 90.0 :`Roll` 90.0) (`self.TileVectorSize`))))
        (`KismetArrayLibrary.Array_AddUnique` (`self.Tiles`) _returnvalue)
        (bind _returnvalue_2 (`AddComponent|NODE_AddTextRenderComponent-0` :`RelativeTransform` (`KismetMathLibrary.MakeTransform` (0.0 0.0 0.0) (struct :`Pitch` 90.0 :`Yaw` 90.0))))
        (bind _returnvalue_3 (`KismetTextLibrary.Conv_IntToText` _index))
        (`TextRenderComponent.K2_SetText` _returnvalue_2 _returnvalue_3)
        (`SceneComponent.K2_AttachToComponent` _returnvalue_2 _returnvalue "None" "KeepRelative" "KeepRelative" "KeepRelative" true)
        (`SceneComponent.SetVisibility` _returnvalue true false)
        (`SceneComponent.SetVisibility` _returnvalue_2 false false)
        (set `ActorComponent.ComponentTags` (`|MakeArray` (`KismetStringLibrary.Conv_StringToName` (`KismetTextLibrary.Conv_TextToString` _returnvalue_3))) _returnvalue)))
    (:`then_1`
      ;[1 1 1] Camera Transform
      (`SceneComponent.K2_SetRelativeTransform` (`self.Camera`) (`self.CameraTransform`) false false))))