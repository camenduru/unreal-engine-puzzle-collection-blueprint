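; Cryptogram puzzle actor where the player decodes a scrambled sentence by clicking letter tiles to type the answer.
; The Construction Script shifts letters by a random offset through a letter DataTable, then spawns the cipher text, answer line and shuffled tile grid with a delete key.
; Activation blends to the puzzle camera and starts a looping timer that outlines hovered tiles via custom depth and recolors text and buttons upon a correct answer.
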(event `/Game/CPCP1/Utilities/Character/Blueprints/BP_PuzzleInterface.DeactivateCamera`
  ;[1 1 1] Exit Puzzle
  (`KismetSystemLibrary.K2_ClearAndInvalidateTimerHandle` (`self.TimerHandle`))
  (for _array_element (`self.Clicables`)
    (`PrimitiveComponent.SetRenderCustomDepth` _array_element false)))

(event `/Game/CPCP1/Utilities/Character/Blueprints/BP_PuzzleInterface.ActivateCamera`
  (bind _returnvalue (`GameplayStatics.GetPlayerController` 0))
  (bind (_returnvalue_x _returnvalue_y) (`KismetMathLibrary.BreakVector2D` (`WidgetLayoutLibrary.GetViewportSize`)))
  (bind _returnvalue_2 (`GameplayStatics.GetPlayerController` 0))
  (bind _returnvalue_3 (`GameplayStatics.GetPlayerController` 0))
  ;[1 1 1] Enter To Puzzle
  (`PlayerController.SetMouseLocation` _returnvalue_2 (`KismetMathLibrary.FTrunc` (/ _returnvalue_x 2.0)) (`KismetMathLibrary.FTrunc` (/ _returnvalue_y 2.0)))
  (`WidgetBlueprintLibrary.SetInputMode_GameAndUIEx` _returnvalue_2 null "DoNotLock" false)
  (`Controller.SetIgnoreLookInput` _returnvalue_3 true)
  (`Controller.SetIgnoreMoveInput` _returnvalue_3 true)
  (`PlayerController.SetViewTargetWithBlend` _returnvalue_3 self 0.5 "VTBlend_Linear" 0.0 false)
  (set `PlayerController.bEnableClickEvents` true _returnvalue)
  (set `PlayerController.bEnableMouseOverEvents` true _returnvalue)
  (set `PlayerController.bShowMouseCursor` true _returnvalue)
  (`WidgetLayoutLibrary.RemoveAllWidgets`)
  ;[1 1 1] Drag And Drop
  (bind _returnvalue_4 (`KismetSystemLibrary.K2_SetTimerDelegate` (delegate `TimerEvent`) (`GameplayStatics.GetWorldDeltaSeconds`) true))
  (set `self.TimerHandle` _returnvalue_4))

(event `TimerEvent`
  (bind _returnvalue (`GameplayStatics.GetPlayerController` 0))
  (bind _hitresult (`PlayerController.GetHitResultUnderCursorForObjects` (`GameplayStatics.GetPlayerController` 0) (`|MakeArray` "ObjectTypeQuery7" :!type "EObjectTypeQuery Enum") true))
  ;[1 1 1] Check Is Puzzle Active
  (bind _asbp_puzzle_character (cast `/Game/CPCP1/Utilities/Character/Blueprints/BP_PuzzleCharacter` (`GameplayStatics.GetPlayerCharacter` 0)))
  (if (`/Game/CPCP1/Utilities/Character/Blueprints/BP_PuzzleCharacter.isPuzzleActive` _asbp_puzzle_character)
    (`|ExecutionSequence`
      (:`then_0`
        ;[1 1 1] Drag And Drop
        (if (`GameplayStatics.BreakHitResult` _hitresult)
          (for _array_element (`self.Clicables`)
            (if (== _array_element (`.HitComponent` (`GameplayStatics.BreakHitResult` _hitresult)))
              (`PrimitiveComponent.SetRenderCustomDepth` _array_element true)
              (set `PlayerController.CurrentMouseCursor` "GrabHand" _returnvalue)
              (for _array_element_2 (`self.Clicables`)
                (if (!= _array_element_2 _array_element)
                  (`PrimitiveComponent.SetRenderCustomDepth` _array_element_2 false)))))
          (else
            (for _array_element_3 (`self.Clicables`) :!label _label
              (`PrimitiveComponent.SetRenderCustomDepth` _array_element_3 false)
              (set `PlayerController.CurrentMouseCursor` "Default" _returnvalue)))))
      (:`then_1`
        ;[1 1 1] Win Condition
        (if (`KismetStringLibrary.EqualEqual_StrStr` (`KismetStringLibrary.ToUpper` (`KismetStringLibrary.TrimTrailing` (`self.EnteredSentence`))) (`KismetStringLibrary.ToUpper` (`KismetStringLibrary.Trim` (`self.CorrectSentence`))))
          (`TextRenderComponent.SetTextRenderColor` (`self.EnterTextComponent`) (make `Color` 0 255))
          (for _array_element_4 (`self.Buttons`)
            (`MeshComponent.SetVectorParameterValueOnMaterials` (break `/Game/CPCP1/Cryptogram/Blueprints/F_CryptogramButton` _array_element_4) "Color" (`KismetMathLibrary.Conv_LinearColorToVector` (`self.WinColor`)))
            (`MeshComponent.SetScalarParameterValueOnMaterials` (break `/Game/CPCP1/Cryptogram/Blueprints/F_CryptogramButton` _array_element_4) "Intensity" (`self.WinIntensity`))))))
    (else
      (goto _label))))

(event `self.ReceiveActorOnClicked`
  (params (ButtonPressed :type "Key Structure"))
  (bind _hitresult (`PlayerController.GetHitResultUnderCursorForObjects` (`GameplayStatics.GetPlayerController` 0) (`|MakeArray` "ObjectTypeQuery7" :!type "EObjectTypeQuery Enum") true))
  ;[1 1 1] Click
  (bind _asbp_puzzle_character (cast `/Game/CPCP1/Utilities/Character/Blueprints/BP_PuzzleCharacter` (`GameplayStatics.GetPlayerCharacter` 0)))
  (if (`/Game/CPCP1/Utilities/Character/Blueprints/BP_PuzzleCharacter.isPuzzleActive` _asbp_puzzle_character)
    (if (`GameplayStatics.BreakHitResult` _hitresult)
      (for _array_element (`self.Clicables`)
        (if (== _array_element (`.HitComponent` (`GameplayStatics.BreakHitResult` _hitresult)))
          (bind _astext_render_component (cast `TextRenderComponent` (`SceneComponent.GetChildComponent` _array_element 0)))
          (bind _text (`TextRenderComponent.Text` _astext_render_component))
          (if (`KismetTextLibrary.NotEqual_TextText` _text (`KismetTextLibrary.Conv_StringToText` (`self.DelButton`)))
            (bind _output_get (set `self.EnteredSentence` (`KismetStringLibrary.Concat_StrStr` (`self.EnteredSentence`) (`KismetTextLibrary.Conv_TextToString` _text))))
            (`TextRenderComponent.K2_SetText` (`self.EnterTextComponent`) (`KismetTextLibrary.Conv_StringToText` _output_get))
            (else
              (bind _output_get_2 (set `self.EnteredSentence` (`KismetStringLibrary.LeftChop` (`self.EnteredSentence`) 1)))
              (`TextRenderComponent.K2_SetText` (`self.EnterTextComponent`) (`KismetTextLibrary.Conv_StringToText` _output_get_2)))))))))

(fn `UserConstructionScript`
  (bind _tilesize (`self.TileSize`))
  (bind _mod (`self.Mod`))
  (`|ExecutionSequence`
    (:`then_0`
      ;[1 1 1] Random Number
      (bind _outrownames (`DataTableFunctionLibrary.GetDataTableRowNames` "/Game/CPCP1/Cryptogram/Blueprints/DT_CryptogramLetterDataTable.DT_CryptogramLetterDataTable"))
      (set `self.RandomNumber` (`KismetMathLibrary.RandomInteger` (`KismetArrayLibrary.Array_Length` _outrownames))))
    (:`then_1`
      ;[1 1 1] Upper and _
      (set `self.CorrectSentence` (`KismetStringLibrary.Replace` (`KismetStringLibrary.ToUpper` (`self.CorrectSentence`)) "" (`self.SpaceCharacter`))))
    (:`then_2`
      ;[1 1 1] Cryptogram
      (for _array_element (`KismetStringLibrary.GetCharacterArrayFromString` (`self.CorrectSentence`))
        (if (`KismetStringLibrary.EqualEqual_StrStr` _array_element (`self.SpaceCharacter`))
          (`KismetArrayLibrary.Array_Add` (`self.MixedSentence`) (`self.SpaceCharacter`))
          (else
            (bind _outrownames_2 (`DataTableFunctionLibrary.GetDataTableRowNames` "/Game/CPCP1/Cryptogram/Blueprints/DT_CryptogramLetterDataTable.DT_CryptogramLetterDataTable"))
            (for (_array_element_2 _array_index) _outrownames_2
              (bind _returnvalue (`|GetDataTableRow` "/Game/CPCP1/Cryptogram/Blueprints/DT_CryptogramLetterDataTable.DT_CryptogramLetterDataTable" _array_element_2)
                (:`then`
                  (if (`KismetStringLibrary.EqualEqual_StrStr` _array_element (`KismetTextLibrary.Conv_TextToString` (break `/Game/CPCP1/Cryptogram/Blueprints/F_CryptogramLetterStruct` _returnvalue)))
                    (bind _outrownames_3 (`DataTableFunctionLibrary.GetDataTableRowNames` "/Game/CPCP1/Cryptogram/Blueprints/DT_CryptogramLetterDataTable.DT_CryptogramLetterDataTable"))
                    (bind _returnvalue_2 (`|GetDataTableRow` "/Game/CPCP1/Cryptogram/Blueprints/DT_CryptogramLetterDataTable.DT_CryptogramLetterDataTable" (`KismetStringLibrary.Conv_StringToName` (`KismetStringLibrary.Conv_IntToString` (mod (+ _array_index (`self.RandomNumber`)) (`KismetArrayLibrary.Array_Length` _outrownames_3)))))
                      (:`then`
                        (`KismetArrayLibrary.Array_Add` (`self.MixedSentence`) (`KismetTextLibrary.Conv_TextToString` (break `/Game/CPCP1/Cryptogram/Blueprints/F_CryptogramLetterStruct` _returnvalue_2)))))))))))))
    (:`then_3`
      (set `self.MixedSentenceString` (`KismetStringLibrary.JoinStringArray` (`self.MixedSentence`))))
    (:`then_4`
      ;[1 1 1] Mixed Sentence
      (bind _returnvalue_3 (`AddComponent|NODE_AddTextRenderComponent-0` :`RelativeTransform` (`KismetMathLibrary.MakeTransform` (0.0 0.0 0.0) (struct :`Pitch` 90.0 :`Yaw` 90.0))))
      (`TextRenderComponent.K2_SetText` _returnvalue_3 (`KismetTextLibrary.Conv_StringToText` (`KismetStringLibrary.ToUpper` (`self.MixedSentenceString`))))
      (`TextRenderComponent.SetWorldSize` _returnvalue_3 (`self.MixedWordSize`))
      (`SceneComponent.K2_AttachToComponent` _returnvalue_3 (`self.Scene`) "None" "KeepRelative" "KeepRelative" "KeepRelative" true))
    (:`then_5`
      ;[1 1 1] Add Tiles And Letters
      (for _array_element_3 (`KismetStringLibrary.GetCharacterArrayFromString` (`self.MixedSentenceString`))
        (`KismetArrayLibrary.Array_AddUnique` (`self.MixedLetters`) _array_element_3)))
    (:`then_6`
      (for _array_element_4 (`KismetStringLibrary.GetCharacterArrayFromString` (`self.CorrectSentence`))
        (`KismetArrayLibrary.Array_AddUnique` (`self.CorrectLetters`) _array_element_4)))
    (:`then_7`
      (`KismetArrayLibrary.Array_Shuffle` (`self.CorrectLetters`))
      (`KismetArrayLibrary.Array_Add` (`self.CorrectLetters`) (`self.DelButton`))
      (for (_array_element_5 _array_index_2) (`self.CorrectLetters`)
        (bind _returnvalue_4 (`AddComponent|NODE_AddStaticMeshComponent-0` :`RelativeTransform` (`KismetMathLibrary.MakeTransform` (`KismetMathLibrary.MakeVector` (`KismetMathLibrary.Conv_IntToDouble` (* (mod _array_index_2 _mod) _tilesize)) (`KismetMathLibrary.Conv_IntToDouble` (* (/ _array_index_2 _mod) _tilesize))) (struct) (`self.ButtonSize`))))
        (`KismetArrayLibrary.Array_AddUnique` (`self.Clicables`) _returnvalue_4)
        (`MeshComponent.SetScalarParameterValueOnMaterials` _returnvalue_4 "Intensity" 1.0)
        (`MeshComponent.SetVectorParameterValueOnMaterials` _returnvalue_4 "Color" (0.0 0.226713 1.0))
        (`PrimitiveComponent.SetCollisionProfileName` _returnvalue_4 "Puzzle" true)
        (bind _returnvalue_5 (`AddComponent|NODE_AddTextRenderComponent-1`))
        (`TextRenderComponent.SetWorldSize` _returnvalue_5 (`self.ButtonWordSize`))
        (`SceneComponent.K2_AttachToComponent` _returnvalue_5 _returnvalue_4 "Text" "SnapToTarget" "SnapToTarget" "KeepRelative" true)
        (`TextRenderComponent.K2_SetText` _returnvalue_5 (`KismetTextLibrary.Conv_StringToText` _array_element_5))
        (`KismetArrayLibrary.Array_Add` (`self.Buttons`) (make `/Game/CPCP1/Cryptogram/Blueprints/F_CryptogramButton` _returnvalue_4 _returnvalue_5 0 _array_element_5))))
    (:`then_8`
      ;[1 1 1] Enter Text
      (bind _returnvalue_6 (`AddComponent|NODE_AddTextRenderComponent-2` :`RelativeTransform` (`KismetMathLibrary.MakeTransform` (`KismetMathLibrary.MakeVector` 0.0 (`self.TypeWordSize`)) (struct :`Pitch` 90.0 :`Yaw` 90.0))))
      (`TextRenderComponent.K2_SetText` _returnvalue_6 (`KismetTextLibrary.Conv_StringToText` ""))
      (`TextRenderComponent.SetWorldSize` _returnvalue_6 (`self.TypeWordSize`))
      (`SceneComponent.K2_AttachToComponent` _returnvalue_6 (`self.Scene`) "None" "KeepRelative" "KeepRelative" "KeepRelative" true)
      (set `self.EnterTextComponent` _returnvalue_6))
    (:`then_9`
      ;[1 1 1] Set Scene Location
      (`SceneComponent.K2_SetRelativeLocation` (`self.Scene`) (`KismetMathLibrary.MakeVector` -12.0 (* (+ (`self.MixedWordSize`) (`self.TypeWordSize`) 5.0) -1.0)) false false))
    (:`then_10`
      ;[1 1 1] Set Camera Position
      (`SceneComponent.K2_SetRelativeTransform` (`self.Camera`) (`self.CameraTransform`) false false))))