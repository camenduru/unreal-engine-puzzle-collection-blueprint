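; BP_SlidePuzzle is a numbered sliding-tile puzzle actor that the player works with the mouse through its own camera.
; The construction script builds a Max×Max board, hides the last tile as the blank, and reshuffles until an inversion-parity check confirms solvability.
; A looping timer highlights hovered tiles, finds neighbors through overlap probes and colors the board by win state.
; Clicking a tile next to the blank swaps the two.
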(event `/Game/CPCP1/Utilities/Character/Blueprints/BP_PuzzleInterface.DeactivateCamera`
  ;[1 1 1] Exit Puzzle
  (`KismetSystemLibrary.K2_ClearAndInvalidateTimerHandle` (`self.TimerHandle`))
  (for _array_element (`self.Mids`)
    (bind _asstatic_mesh_component (cast `StaticMeshComponent` _array_element))
    (`PrimitiveComponent.SetRenderCustomDepth` _asstatic_mesh_component false)))

(event `/Game/CPCP1/Utilities/Character/Blueprints/BP_PuzzleInterface.ActivateCamera`
  (bind _returnvalue (`GameplayStatics.GetPlayerController` 0))
  (bind (_returnvalue_x _returnvalue_y) (`KismetMathLibrary.BreakVector2D` (`WidgetLayoutLibrary.GetViewportSize`)))
  (bind _returnvalue_2 (`GameplayStatics.GetPlayerController` 0))
  (bind _returnvalue_3 (`GameplayStatics.GetPlayerController` 0))
  ;[1 1 1] Enter To Puzzle
  (`PlayerController.SetMouseLocation` _returnvalue_2 (`KismetMathLibrary.FTrunc` (/ _returnvalue_x 2.0)) (`KismetMathLibrary.FTrunc` (/ _returnvalue_y 2.0)))
  (`WidgetBlueprintLibrary.SetInputMode_GameAndUIEx` _returnvalue_2 null "DoNotLock" false)
  (`Controller.SetIgnoreLookInput` _returnvalue_3 true)
  (`Controller.SetIgnoreMoveInput` _returnvalue_3 true)
  (`PlayerController.SetViewTargetWithBlend` _returnvalue_3 self 0.5 "VTBlend_Linear" 0.0 false)
  (set `PlayerController.bEnableClickEvents` true _returnvalue)
  (set `PlayerController.bEnableMouseOverEvents` true _returnvalue)
  (set `PlayerController.bShowMouseCursor` true _returnvalue)
  (`WidgetLayoutLibrary.RemoveAllWidgets`)
  (bind _returnvalue_4 (`KismetSystemLibrary.K2_SetTimerDelegate` (delegate `TimerEvent`) (`GameplayStatics.GetWorldDeltaSeconds`) true))
  (set `self.TimerHandle` _returnvalue_4))

(event `TimerEvent`
  (bind _returnvalue (`GameplayStatics.GetPlayerController` 0))
  (bind _tiles (`self.Tiles`))
  (bind _hitresult (`PlayerController.GetHitResultUnderCursorForObjects` (`GameplayStatics.GetPlayerController` 0) (`|MakeArray` "ObjectTypeQuery7" :!type "EObjectTypeQuery Enum") false))
  ;[1 1 1] Check Is Puzzle Active
  (bind _asbp_puzzle_character (cast `/Game/CPCP1/Utilities/Character/Blueprints/BP_PuzzleCharacter` (`GameplayStatics.GetPlayerCharacter` 0)))
  (if (`/Game/CPCP1/Utilities/Character/Blueprints/BP_PuzzleCharacter.isPuzzleActive` _asbp_puzzle_character)
    (`|ExecutionSequence`
      (:`then_0`
        ;[1 1 1] Drag And Drop
        (if (`GameplayStatics.BreakHitResult` _hitresult)
          (for _array_element (`self.Mids`)
            (bind _asstatic_mesh_component (cast `StaticMeshComponent` _array_element))
            (if (== _asstatic_mesh_component (`.HitComponent` (`GameplayStatics.BreakHitResult` _hitresult)))
              (`PrimitiveComponent.SetRenderCustomDepth` _asstatic_mesh_component true)
              (set `PlayerController.CurrentMouseCursor` "GrabHand" _returnvalue)
              (for _array_element_2 (`self.Mids`)
                (bind _asstatic_mesh_component_2 (cast `StaticMeshComponent` _array_element_2))
                (if (!= _asstatic_mesh_component_2 _asstatic_mesh_component)
                  (`PrimitiveComponent.SetRenderCustomDepth` _asstatic_mesh_component_2 false)))))
          (else
            (for _array_element_3 (`self.Mids`) :!label _label
              (bind _asstatic_mesh_component_3 (cast `StaticMeshComponent` _array_element_3))
              (`PrimitiveComponent.SetRenderCustomDepth` _asstatic_mesh_component_3 false)
              (set `PlayerController.CurrentMouseCursor` "Default" _returnvalue)))))
      (:`then_1`
        ;[1 1 1] Init
        (for _array_element_4 (`self.Tiles`)
          (`|ExecutionSequence`
            (:`then_0`
              (bind _output (`|GetArrayItem` (`self.GetComponentsByTag` "/Script/Engine.StaticMeshComponent" (`KismetStringLibrary.Conv_StringToName` (`KismetStringLibrary.Concat_StrStr` "W" (`KismetStringLibrary.Conv_IntToString` (`.Id_11_D6BE633341B87639E437B3ADAFED5821` (break `/Game/CPCP1/Slide/Blueprints/F_Tile` _array_element_4))))))))
              (bind _outcomponents (`KismetSystemLibrary.ComponentOverlapComponents` _output (`SceneComponent.K2_GetComponentToWorld` _output) (`|MakeArray` "ObjectTypeQuery1" :!type "EObjectTypeQuery Enum") "/Script/Engine.StaticMeshComponent"))
              (if (`KismetArrayLibrary.Array_IsNotEmpty` _outcomponents)
                (bind _output_w (break `/Game/CPCP1/Slide/Blueprints/F_Tile` (`|GetArrayItem` (`self.Tiles`) (- (`.Id_11_D6BE633341B87639E437B3ADAFED5821` (break `/Game/CPCP1/Slide/Blueprints/F_Tile` _array_element_4)) 1))))
                (`|VariableSetRef` _output_w (`KismetStringLibrary.Conv_StringToInt` (`KismetStringLibrary.Conv_NameToString` (`|GetArrayItem` (`ActorComponent.ComponentTags` (`SceneComponent.GetAttachParent` (`|GetArrayItem` _outcomponents)))))))
                (else
                  (`|VariableSetRef` _output_w))))
            (:`then_1`
              (bind _output_2 (`|GetArrayItem` (`self.GetComponentsByTag` "/Script/Engine.StaticMeshComponent" (`KismetStringLibrary.Conv_StringToName` (`KismetStringLibrary.Concat_StrStr` "N" (`KismetStringLibrary.Conv_IntToString` (`.Id_11_D6BE633341B87639E437B3ADAFED5821` (break `/Game/CPCP1/Slide/Blueprints/F_Tile` _array_element_4))))))))
              (bind _outcomponents_2 (`KismetSystemLibrary.ComponentOverlapComponents` _output_2 (`SceneComponent.K2_GetComponentToWorld` _output_2) (`|MakeArray` "ObjectTypeQuery1" :!type "EObjectTypeQuery Enum") "/Script/Engine.StaticMeshComponent"))
              (if (`KismetArrayLibrary.Array_IsNotEmpty` _outcomponents_2)
                (bind (_output_w_2 _output_n) (break `/Game/CPCP1/Slide/Blueprints/F_Tile` (`|GetArrayItem` (`self.Tiles`) (- (`.Id_11_D6BE633341B87639E437B3ADAFED5821` (break `/Game/CPCP1/Slide/Blueprints/F_Tile` _array_element_4)) 1))))
                (`|VariableSetRef` _output_n (`KismetStringLibrary.Conv_StringToInt` (`KismetStringLibrary.Conv_NameToString` (`|GetArrayItem` (`ActorComponent.ComponentTags` (`SceneComponent.GetAttachParent` (`|GetArrayItem` _outcomponents_2)))))))
                (else
                  (`|VariableSetRef` _output_n))))
            (:`then_2`
              (bind _output_3 (`|GetArrayItem` (`self.GetComponentsByTag` "/Script/Engine.StaticMeshComponent" (`KismetStringLibrary.Conv_StringToName` (`KismetStringLibrary.Concat_StrStr` "E" (`KismetStringLibrary.Conv_IntToString` (`.Id_11_D6BE633341B87639E437B3ADAFED5821` (break `/Game/CPCP1/Slide/Blueprints/F_Tile` _array_element_4))))))))
              (bind _outcomponents_3 (`KismetSystemLibrary.ComponentOverlapComponents` _output_3 (`SceneComponent.K2_GetComponentToWorld` _output_3) (`|MakeArray` "ObjectTypeQuery1" :!type "EObjectTypeQuery Enum") "/Script/Engine.StaticMeshComponent"))
              (if (`KismetArrayLibrary.Array_IsNotEmpty` _outcomponents_3)
                (bind (_output_w_3 _output_n_2 _output_e) (break `/Game/CPCP1/Slide/Blueprints/F_Tile` (`|GetArrayItem` (`self.Tiles`) (- (`.Id_11_D6BE633341B87639E437B3ADAFED5821` (break `/Game/CPCP1/Slide/Blueprints/F_Tile` _array_element_4)) 1))))
                (`|VariableSetRef` _output_e (`KismetStringLibrary.Conv_StringToInt` (`KismetStringLibrary.Conv_NameToString` (`|GetArrayItem` (`ActorComponent.ComponentTags` (`SceneComponent.GetAttachParent` (`|GetArrayItem` _outcomponents_3)))))))
                (else
                  (`|VariableSetRef` _output_e))))
            (:`then_3`
              (bind _output_4 (`|GetArrayItem` (`self.GetComponentsByTag` "/Script/Engine.StaticMeshComponent" (`KismetStringLibrary.Conv_StringToName` (`KismetStringLibrary.Concat_StrStr` "S" (`KismetStringLibrary.Conv_IntToString` (`.Id_11_D6BE633341B87639E437B3ADAFED5821` (break `/Game/CPCP1/Slide/Blueprints/F_Tile` _array_element_4))))))))
              (bind _outcomponents_4 (`KismetSystemLibrary.ComponentOverlapComponents` _output_4 (`SceneComponent.K2_GetComponentToWorld` _output_4) (`|MakeArray` "ObjectTypeQuery1" :!type "EObjectTypeQuery Enum") "/Script/Engine.StaticMeshComponent"))
              (if (`KismetArrayLibrary.Array_IsNotEmpty` _outcomponents_4)
                (bind (_output_w_4 _output_n_3 _output_e_2 _output_s) (break `/Game/CPCP1/Slide/Blueprints/F_Tile` (`|GetArrayItem` (`self.Tiles`) (- (`.Id_11_D6BE633341B87639E437B3ADAFED5821` (break `/Game/CPCP1/Slide/Blueprints/F_Tile` _array_element_4)) 1))))
                (`|VariableSetRef` _output_s (`KismetStringLibrary.Conv_StringToInt` (`KismetStringLibrary.Conv_NameToString` (`|GetArrayItem` (`ActorComponent.ComponentTags` (`SceneComponent.GetAttachParent` (`|GetArrayItem` _outcomponents_4)))))))
                (else
                  (`|VariableSetRef` _output_s)))))))
      (:`then_2`
        ;[1 1 1] Win Condition
        (for _array_element_5 _tiles
          (set `self.SlidePuzzleWin` false)
          (if (== (`.Id_11_D6BE633341B87639E437B3ADAFED5821` (break `/Game/CPCP1/Slide/Blueprints/F_Tile` _array_element_5)) (`.Position_12_35554ADB40BF7552F5896882FE435E24` (break `/Game/CPCP1/Slide/Blueprints/F_Tile` _array_element_5)))
            (set `self.SlidePuzzleWin` true)
            (else
              (break)))))
      (:`then_3`
        (if (`self.SlidePuzzleWin`)
          (for _array_element_6 _tiles
            (bind _asmesh_component (cast `MeshComponent` (`.Piece_18_B2DBFFFC426CF2A026EC71894D335B86` (break `/Game/CPCP1/Slide/Blueprints/F_Tile` _array_element_6))))
            (`MeshComponent.SetVectorParameterValueOnMaterials` _asmesh_component "Color" (0.0 1.0 0.0))
            (`MeshComponent.SetScalarParameterValueOnMaterials` _asmesh_component "Intensity" 10.0))
          (else
            (for _array_element_7 _tiles
              (bind _asmesh_component_2 (cast `MeshComponent` (`.Piece_18_B2DBFFFC426CF2A026EC71894D335B86` (break `/Game/CPCP1/Slide/Blueprints/F_Tile` _array_element_7))))
              (`MeshComponent.SetVectorParameterValueOnMaterials` _asmesh_component_2 "Color" (1.0 0.0 0.0))
              (`MeshComponent.SetScalarParameterValueOnMaterials` _asmesh_component_2 "Intensity" 10.0))))))
    (else
      (goto _label))))

(event `self.ReceiveActorOnClicked`
  (params (ButtonPressed :type "Key Structure"))
  (bind _tiles (`self.Tiles`))
  (bind _hitresult (`PlayerController.GetHitResultUnderCursorForObjects` (`GameplayStatics.GetPlayerController` 0) (`|MakeArray` "ObjectTypeQuery7" :!type "EObjectTypeQuery Enum") true))
  (bind (_output_w _output_n _output_e _output_s _output_id _output_position _output_piece) (break `/Game/CPCP1/Slide/Blueprints/F_Tile` (`|GetArrayItem` _tiles (- (`KismetArrayLibrary.Array_Length` _tiles) 1))))
  ;[1 1 1] Click
  (bind _asbp_puzzle_character (cast `/Game/CPCP1/Utilities/Character/Blueprints/BP_PuzzleCharacter` (`GameplayStatics.GetPlayerCharacter` 0)))
  (if (`/Game/CPCP1/Utilities/Character/Blueprints/BP_PuzzleCharacter.isPuzzleActive` _asbp_puzzle_character)
    (if (`GameplayStatics.BreakHitResult` _hitresult)
      (for _array_element (`self.Mids`)
        (bind _asstatic_mesh_component (cast `StaticMeshComponent` _array_element))
        (if (== _asstatic_mesh_component (`.HitComponent` (`GameplayStatics.BreakHitResult` _hitresult)))
          (if (== (`|GetArrayItem` (`ActorComponent.ComponentTags` _asstatic_mesh_component)) "Mid")
            (bind (_output_w_2 _output_n_2 _output_e_2 _output_s_2 _output_id_2 _output_position_2 _output_piece_2) (break `/Game/CPCP1/Slide/Blueprints/F_Tile` (`|GetArrayItem` _tiles (- (`KismetStringLibrary.Conv_StringToInt` (`KismetStringLibrary.Conv_NameToString` (`|GetArrayItem` (`ActorComponent.ComponentTags` (`SceneComponent.GetAttachParent` _asstatic_mesh_component))))) 1))))
            (if (or (== _output_w_2 _output_id) (== _output_n_2 _output_id) (== _output_e_2 _output_id) (== _output_s_2 _output_id))
              (bind _asmesh_component (cast `MeshComponent` _output_piece))
              (set `self.TempTransformEmpty` (`SceneComponent.K2_GetComponentToWorld` _asmesh_component))
              (set `self.TempPositionEmpty` _output_position)
              (bind _asmesh_component_2 (cast `MeshComponent` _output_piece_2))
              (set `self.TempTransform` (`SceneComponent.K2_GetComponentToWorld` _asmesh_component_2))
              (set `self.TempPosition` _output_position_2)
              (`SceneComponent.K2_SetWorldTransform` _asmesh_component_2 (`self.TempTransformEmpty`) false false)
              (`|VariableSetRef` _output_position_2 (`self.TempPositionEmpty`))
              (`SceneComponent.K2_SetWorldTransform` _asmesh_component (`self.TempTransform`) false false)
              (`|VariableSetRef` _output_position (`self.TempPosition`)))))))))

(fn `CountInversions`
  (params (Array :type "Array of Integer") (Max :type Integer) (Except :type Integer))
  (returns (Total :type Integer))
  (locals (Counter :type Integer))
  ;[1 1 1] Inversion Count
  (`|ExecutionSequence`
    (:`then_0`
      (set `local.Counter` 0))
    (:`then_1`
      (for _index (range (+ (- (* Max Max) 2) 1))
        (for _index_2 (range (+ _index 1) (* Max Max))
          (if (and (!= (`|GetArrayItem` Array _index_2) Except) (!= (`|GetArrayItem` Array _index) Except) (> (`|GetArrayItem` Array _index) (`|GetArrayItem` Array _index_2)))
            (`/Engine/EditorBlueprintResources/StandardMacros.IncrementInt` (`local.Counter`))))))
    (:`then_2`
      (return (`local.Counter`)))))

(fn `UserConstructionScript`
  (bind _tilesize (`self.TileSize`))
  (bind _tiles (`self.Tiles`))
  (bind _max (`self.Max`))
  (bind _tiles_2 (`self.Tiles`))
  (bind _max_2 (`self.Max`))
  (bind _returnvalue (* (`self.Max`) (`self.Max`)))
  (bind _returnvalue_2 (== (mod (`self.Max`) 2) 0))
  (bind (_output_w _output_n _output_e _output_s _output_id _output_position _output_piece _output_text _output_mid) (break `/Game/CPCP1/Slide/Blueprints/F_Tile` (`|GetArrayItem` _tiles_2 (- (`KismetArrayLibrary.Array_Length` _tiles_2) 1))))
  (`|ExecutionSequence`
    (:`then_0`
      ;[1 1 1] Clear Tiles
      (`KismetArrayLibrary.Array_Clear` (`self.Tiles`)))
    (:`then_1`
      ;[1 1 1] Set Board
      (for _index (range (* _max _max))
        (bind _returnvalue_3 (`AddComponent|NODE_AddStaticMeshComponent-0` :`RelativeTransform` (`KismetMathLibrary.MakeTransform` (`KismetMathLibrary.MakeVector` (`KismetMathLibrary.Conv_IntToDouble` (* (mod _index _max) _tilesize)) (`KismetMathLibrary.Conv_IntToDouble` (* (/ _index _max) _tilesize))) (struct) (0.1 0.1 0.1))))
        (`MeshComponent.SetScalarParameterValueOnMaterials` _returnvalue_3 "Intensity" 1.0)
        (bind _returnvalue_4 (`AddComponent|NODE_AddTextRenderComponent-0`))
        (`TextRenderComponent.K2_SetText` _returnvalue_4 (`KismetTextLibrary.Conv_IntToText` (+ _index 1)))
        (`TextRenderComponent.SetWorldSize` _returnvalue_4 200.0)
        (`SceneComponent.K2_AttachToComponent` _returnvalue_4 _returnvalue_3 "Text" "KeepRelative" "KeepRelative" "KeepRelative" true)
        (bind _returnvalue_5 (`AddComponent|NODE_AddStaticMeshComponent-6`))
        (`KismetArrayLibrary.Array_AddUnique` (`self.Mids`) _returnvalue_5)
        (set `ActorComponent.ComponentTags` (`|MakeArray` "Mid" :!type "Name") _returnvalue_5)
        (`SceneComponent.SetVisibility` _returnvalue_5 true false)
        (`PrimitiveComponent.SetCollisionProfileName` _returnvalue_5 "Puzzle" true)
        (`MeshComponent.SetScalarParameterValueOnMaterials` _returnvalue_5 "Intensity" 0.0)
        (`SceneComponent.K2_AttachToComponent` _returnvalue_5 _returnvalue_3 "Mid" "KeepRelative" "KeepRelative" "KeepRelative" true)
        (bind _returnvalue_6 (+ _index 1))
        (set `ActorComponent.ComponentTags` (`|MakeArray` (`KismetStringLibrary.Conv_StringToName` (`KismetStringLibrary.Conv_IntToString` _returnvalue_6))) _returnvalue_3)
        (`KismetArrayLibrary.Array_AddUnique` (`self.Tiles`) (make `/Game/CPCP1/Slide/Blueprints/F_Tile` 0 0 0 0 _returnvalue_6 _returnvalue_6 _returnvalue_3 _returnvalue_4 _returnvalue_5))
        (`|ExecutionSequence`
          (:`then_0`
            (bind _returnvalue_7 (`AddComponent|NODE_AddStaticMeshComponent-1`))
            (`SceneComponent.SetVisibility` _returnvalue_7 false false)
            (`PrimitiveComponent.SetCollisionProfileName` _returnvalue_7 "OverlapAll" true)
            (set `ActorComponent.ComponentTags` (`|MakeArray` (`KismetStringLibrary.Conv_StringToName` (`KismetStringLibrary.Concat_StrStr` "W" (`KismetStringLibrary.Conv_IntToString` _returnvalue_6)))) _returnvalue_7)
            (`SceneComponent.K2_AttachToComponent` _returnvalue_7 _returnvalue_3 "W" "KeepRelative" "KeepRelative" "KeepRelative" true))
          (:`then_1`
            (bind _returnvalue_8 (`AddComponent|NODE_AddStaticMeshComponent-2`))
            (`SceneComponent.SetVisibility` _returnvalue_8 false false)
            (`PrimitiveComponent.SetCollisionProfileName` _returnvalue_8 "OverlapAll" true)
            (set `ActorComponent.ComponentTags` (`|MakeArray` (`KismetStringLibrary.Conv_StringToName` (`KismetStringLibrary.Concat_StrStr` "N" (`KismetStringLibrary.Conv_IntToString` _returnvalue_6)))) _returnvalue_8)
            (`SceneComponent.K2_AttachToComponent` _returnvalue_8 _returnvalue_3 "N" "KeepRelative" "KeepRelative" "KeepRelative" true))
          (:`then_2`
            (bind _returnvalue_9 (`AddComponent|NODE_AddStaticMeshComponent-3`))
            (`SceneComponent.SetVisibility` _returnvalue_9 false false)
            (`PrimitiveComponent.SetCollisionProfileName` _returnvalue_9 "OverlapAll" true)
            (set `ActorComponent.ComponentTags` (`|MakeArray` (`KismetStringLibrary.Conv_StringToName` (`KismetStringLibrary.Concat_StrStr` "E" (`KismetStringLibrary.Conv_IntToString` _returnvalue_6)))) _returnvalue_9)
            (`SceneComponent.K2_AttachToComponent` _returnvalue_9 _returnvalue_3 "E" "KeepRelative" "KeepRelative" "KeepRelative" true))
          (:`then_3`
            (bind _returnvalue_10 (`AddComponent|NODE_AddStaticMeshComponent-4`))
            (`SceneComponent.SetVisibility` _returnvalue_10 false false)
            (`PrimitiveComponent.SetCollisionProfileName` _returnvalue_10 "OverlapAll" true)
            (set `ActorComponent.ComponentTags` (`|MakeArray` (`KismetStringLibrary.Conv_StringToName` (`KismetStringLibrary.Concat_StrStr` "S" (`KismetStringLibrary.Conv_IntToString` _returnvalue_6)))) _returnvalue_10)
            (`SceneComponent.K2_AttachToComponent` _returnvalue_10 _returnvalue_3 "S" "KeepRelative" "KeepRelative" "KeepRelative" true)))))
    (:`then_2`
      ;[1 1 1] Hide Last Tile
      (bind _asstatic_mesh_component (cast `StaticMeshComponent` _output_piece))
      (`SceneComponent.SetVisibility` _asstatic_mesh_component false false)
      (`SceneComponent.SetVisibility` _output_text false false)
      (bind _asstatic_mesh_component_2 (cast `StaticMeshComponent` _output_mid))
      (`SceneComponent.SetVisibility` _asstatic_mesh_component_2 false false))
    (:`then_3`
      ;[1 1 1] Mix The Puzzle
      (`|ExecutionSequence`
        (:`then_0`
          ;;[1 1 1] Add Reverse Rows
          (for _index_2 (range 1 (+ (`self.Max`) 1))
            (`KismetArrayLibrary.Array_AddUnique` (`self.ReverseRows`) _index_2)))
        (:`then_1`
          (`KismetArrayLibrary.Array_Reverse` (`self.ReverseRows`)))
        (:`then_2`
          ;;[1 1 1] Mix
          (set `self.InversionCount` 0)
          (`KismetArrayLibrary.Array_Clear` (`self.MixedPositions`)))
        (:`then_3`
          (for _index_3 (range (* (`self.Max`) (`self.Max`)))
            (`KismetArrayLibrary.Array_AddUnique` (`self.MixedPositions`) (+ _index_3 1))))
        (:`then_4`
          ;;[1 1 1] Is Solvable
          (`KismetArrayLibrary.Array_Shuffle` (`self.MixedPositions`) :!label _label)
          (bind _total (`self.CountInversions` (`self.MixedPositions`) (`self.Max`) (* (`self.Max`) (`self.Max`))))
          (set `self.InversionCount` _total)
          ;;[1 1 1] http://kevingong.com/Math/SixteenPuzzle.html
          ;; https://web.archive.org/web/20180617081657/https://www.cs.bham.ac.uk/~mdr/teaching/modules04/java2/TilesSolvability.html
          ;; If the grid width is odd, then the number of inversions in a solvable situation is even.
          ;; If the grid width is even, and the blank is on an even row counting from the bottom (second-last, fourth-last etc), then the number of inversions in a solvable situation is odd.
          ;; If the grid width is even, and the blank is on an odd row counting from the bottom (last, third-last, fifth-last etc) then the number of inversions in a solvable situation is even.
          (if (not (or (and (!= (mod (`self.Max`) 2) 0) (== (mod (`self.InversionCount`) 2) 0)) (and _returnvalue_2 (and (!= (mod (`|GetArrayItem` (`self.ReverseRows`) (/ (`KismetArrayLibrary.Array_Find` (`self.MixedPositions`) _returnvalue) _max_2)) 2) 0) (== (mod (`self.InversionCount`) 2) 0))) (and _returnvalue_2 (and (== (mod (`|GetArrayItem` (`self.ReverseRows`) (/ (`KismetArrayLibrary.Array_Find` (`self.MixedPositions`) _returnvalue) _max_2)) 2) 0) (!= (mod (`self.InversionCount`) 2) 0)))))
            (goto _label)))))
    (:`then_4`
      ;[1 1 1] Plot
      (`|ExecutionSequence`
        (:`then_0`
          (`BlueprintMapLibrary.Map_Clear` (`self.MixedPositionMap`)))
        (:`then_1`
          (for _array_element (`self.Tiles`)
            (bind _asmesh_component (cast `MeshComponent` (`.Piece_18_B2DBFFFC426CF2A026EC71894D335B86` (break `/Game/CPCP1/Slide/Blueprints/F_Tile` _array_element))))
            (`BlueprintMapLibrary.Map_Add` (`self.MixedPositionMap`) (`.Position_12_35554ADB40BF7552F5896882FE435E24` (break `/Game/CPCP1/Slide/Blueprints/F_Tile` _array_element)) (`SceneComponent.K2_GetComponentToWorld` _asmesh_component))))
        (:`then_2`
          (for (_array_element_2 _array_index) (`self.MixedPositions`)
            (bind _values (`BlueprintMapLibrary.Map_Values` (`self.MixedPositionMap`)))
            (for (_array_element_3 _array_index_2) (`self.Tiles`)
              (if (== (`.Position_12_35554ADB40BF7552F5896882FE435E24` (break `/Game/CPCP1/Slide/Blueprints/F_Tile` _array_element_3)) _array_element_2)
                (`KismetArrayLibrary.Array_AddUnique` (`self.MixedTiles`) _array_index_2)
                (bind _asmesh_component_2 (cast `MeshComponent` (`.Piece_18_B2DBFFFC426CF2A026EC71894D335B86` (break `/Game/CPCP1/Slide/Blueprints/F_Tile` _array_element_3))))
                (`SceneComponent.K2_SetWorldTransform` _asmesh_component_2 (`|GetArrayItem` _values _array_index) false false)))))
        (:`then_3`
          (for (_array_element_4 _array_index_3) (`self.MixedTiles`)
            (bind (_output_w_2 _output_n_2 _output_e_2 _output_s_2 _output_id_2 _output_position_2 _output_piece_2 _output_text_2 _output_mid_2) (break `/Game/CPCP1/Slide/Blueprints/F_Tile` (`|GetArrayItem` _tiles _array_element_4)))
            (`KismetArrayLibrary.Array_Set` _tiles _array_element_4 (make `/Game/CPCP1/Slide/Blueprints/F_Tile` _output_w_2 _output_n_2 _output_e_2 _output_s_2 _output_id_2 (+ _array_index_3 1) _output_piece_2 _output_text_2 _output_mid_2))))))
    (:`then_5`
      ;[1 1 1] Set Camera Position
      (`SceneComponent.K2_SetRelativeTransform` (`self.Camera`) (`self.CameraTransform`) false false))))