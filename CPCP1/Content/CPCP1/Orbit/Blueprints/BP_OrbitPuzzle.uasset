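; BP_OrbitPuzzle is a camera-view puzzle where clicking one of three buttons rotates nearby orbiters 60 degrees around it.
; The construction script colors red and green pieces and lays them out on overlapping hexagonal rings.
; While active, a per-frame looping timer highlights hovered buttons with custom depth.
; It also checks whether green orbiters cover the six target positions (three toruses, three buttons), then brightens the materials on a win.
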(event `/Game/CPCP1/Utilities/Character/Blueprints/BP_PuzzleInterface.DeactivateCamera`
  ;[1 1 1] Exit Puzzle
  (`KismetSystemLibrary.K2_ClearAndInvalidateTimerHandle` (`self.TimerHandle`))
  (for _array_element (`self.Pieces`)
    (bind _asstatic_mesh_component (cast `StaticMeshComponent` _array_element))
    (`PrimitiveComponent.SetRenderCustomDepth` _asstatic_mesh_component false)))

(event `/Game/CPCP1/Utilities/Character/Blueprints/BP_PuzzleInterface.ActivateCamera`
  (bind _returnvalue (`GameplayStatics.GetPlayerController` 0))
  (bind (_returnvalue_x _returnvalue_y) (`KismetMathLibrary.BreakVector2D` (`WidgetLayoutLibrary.GetViewportSize`)))
  (bind _returnvalue_2 (`GameplayStatics.GetPlayerController` 0))
  (bind _returnvalue_3 (`GameplayStatics.GetPlayerController` 0))
  ;[1 1 1] Enter To Puzzle
  (`PlayerController.SetMouseLocation` _returnvalue_2 (`KismetMathLibrary.FTrunc` (/ _returnvalue_x 2.0)) (`KismetMathLibrary.FTrunc` (/ _returnvalue_y 2.0)))
  (`WidgetBlueprintLibrary.SetInputMode_GameAndUIEx` _returnvalue_2 null "DoNotLock" false)
  (`Controller.SetIgnoreLookInput` _returnvalue_3 true)
  (`Controller.SetIgnoreMoveInput` _returnvalue_3 true)
  (`PlayerController.SetViewTargetWithBlend` _returnvalue_3 self 0.5 "VTBlend_Linear" 0.0 false)
  (set `PlayerController.bEnableClickEvents` true _returnvalue)
  (set `PlayerController.bEnableMouseOverEvents` true _returnvalue)
  (set `PlayerController.bShowMouseCursor` true _returnvalue)
  (`WidgetLayoutLibrary.RemoveAllWidgets`)
  ;[1 1 1] Drag And Drop
  (bind _returnvalue_4 (`KismetSystemLibrary.K2_SetTimerDelegate` (delegate `TimerEvent`) (`GameplayStatics.GetWorldDeltaSeconds`) true))
  (set `self.TimerHandle` _returnvalue_4))

(event `TimerEvent`
  (bind _returnvalue (`GameplayStatics.GetPlayerController` 0))
  (bind _tolerance (`self.Tolerance`))
  (bind _tolerance_2 (`self.Tolerance`))
  (bind _tolerance_3 (`self.Tolerance`))
  (bind _tolerance_4 (`self.Tolerance`))
  (bind _tolerance_5 (`self.Tolerance`))
  (bind _tolerance_6 (`self.Tolerance`))
  (bind _hitresult (`PlayerController.GetHitResultUnderCursorForObjects` (`GameplayStatics.GetPlayerController` 0) (`|MakeArray` "ObjectTypeQuery7" :!type "EObjectTypeQuery Enum") true))
  (bind _relativelocation (`SceneComponent.RelativeLocation` (`self.ButtonLeft`)))
  (bind _relativelocation_2 (`SceneComponent.RelativeLocation` (`self.Torus3`)))
  (bind _relativelocation_3 (`SceneComponent.RelativeLocation` (`self.Torus2`)))
  (bind _relativelocation_4 (`SceneComponent.RelativeLocation` (`self.Torus1`)))
  (bind _relativelocation_5 (`SceneComponent.RelativeLocation` (`self.ButtonUp`)))
  (bind _relativelocation_6 (`SceneComponent.RelativeLocation` (`self.ButtonRight`)))
  ;[1 1 1] Check Is Puzzle Active
  (bind _asbp_puzzle_character (cast `/Game/CPCP1/Utilities/Character/Blueprints/BP_PuzzleCharacter` (`GameplayStatics.GetPlayerCharacter` 0)))
  (if (`/Game/CPCP1/Utilities/Character/Blueprints/BP_PuzzleCharacter.isPuzzleActive` _asbp_puzzle_character)
    (`|ExecutionSequence`
      (:`then_0`
        ;[1 1 1] Drag And Drop
        (if (`GameplayStatics.BreakHitResult` _hitresult)
          (for _array_element (`self.Pieces`)
            (bind _asstatic_mesh_component (cast `StaticMeshComponent` _array_element))
            (if (== _array_element (`.HitComponent` (`GameplayStatics.BreakHitResult` _hitresult)))
              (`PrimitiveComponent.SetRenderCustomDepth` _asstatic_mesh_component true)
              (set `PlayerController.CurrentMouseCursor` "GrabHand" _returnvalue)
              (for _array_element_2 (`self.Pieces`)
                (bind _asstatic_mesh_component_2 (cast `StaticMeshComponent` _array_element_2))
                (if (!= _asstatic_mesh_component_2 _asstatic_mesh_component)
                  (`PrimitiveComponent.SetRenderCustomDepth` _asstatic_mesh_component_2 false)))))
          (else
            (for _array_element_3 (`self.Pieces`) :!label _label
              (bind _asstatic_mesh_component_3 (cast `StaticMeshComponent` _array_element_3))
              (`PrimitiveComponent.SetRenderCustomDepth` _asstatic_mesh_component_3 false)
              (set `PlayerController.CurrentMouseCursor` "Default" _returnvalue)))))
      (:`then_1`
        ;[1 1 1] Win Condition
        (if (and (or (== _relativelocation_2 (`SceneComponent.RelativeLocation` (`self.Orbiter0`)) :`ErrorTolerance` _tolerance_2) (== _relativelocation_2 (`SceneComponent.RelativeLocation` (`self.Orbiter2`)) :`ErrorTolerance` _tolerance_2) (== _relativelocation_2 (`SceneComponent.RelativeLocation` (`self.Orbiter4`)) :`ErrorTolerance` _tolerance_2) (== _relativelocation_2 (`SceneComponent.RelativeLocation` (`self.Orbiter9`)) :`ErrorTolerance` _tolerance_2) (== _relativelocation_2 (`SceneComponent.RelativeLocation` (`self.Orbiter10`)) :`ErrorTolerance` _tolerance_2) (== _relativelocation_2 (`SceneComponent.RelativeLocation` (`self.Orbiter11`)) :`ErrorTolerance` _tolerance_2)) (or (== _relativelocation_3 (`SceneComponent.RelativeLocation` (`self.Orbiter0`)) :`ErrorTolerance` _tolerance_3) (== _relativelocation_3 (`SceneComponent.RelativeLocation` (`self.Orbiter2`)) :`ErrorTolerance` _tolerance_3) (== _relativelocation_3 (`SceneComponent.RelativeLocation` (`self.Orbiter4`)) :`ErrorTolerance` _tolerance_3) (== _relativelocation_3 (`SceneComponent.RelativeLocation` (`self.Orbiter9`)) :`ErrorTolerance` _tolerance_3) (== _relativelocation_3 (`SceneComponent.RelativeLocation` (`self.Orbiter10`)) :`ErrorTolerance` _tolerance_3) (== _relativelocation_3 (`SceneComponent.RelativeLocation` (`self.Orbiter11`)) :`ErrorTolerance` _tolerance_3)) (or (== _relativelocation_4 (`SceneComponent.RelativeLocation` (`self.Orbiter0`)) :`ErrorTolerance` _tolerance_4) (== _relativelocation_4 (`SceneComponent.RelativeLocation` (`self.Orbiter2`)) :`ErrorTolerance` _tolerance_4) (== _relativelocation_4 (`SceneComponent.RelativeLocation` (`self.Orbiter4`)) :`ErrorTolerance` _tolerance_4) (== _relativelocation_4 (`SceneComponent.RelativeLocation` (`self.Orbiter9`)) :`ErrorTolerance` _tolerance_4) (== _relativelocation_4 (`SceneComponent.RelativeLocation` (`self.Orbiter10`)) :`ErrorTolerance` _tolerance_4) (== _relativelocation_4 (`SceneComponent.RelativeLocation` (`self.Orbiter11`)) :`ErrorTolerance` _tolerance_4)) (or (== _relativelocation_5 (`SceneComponent.RelativeLocation` (`self.Orbiter0`)) :`ErrorTolerance` _tolerance_5) (== _relativelocation_5 (`SceneComponent.RelativeLocation` (`self.Orbiter2`)) :`ErrorTolerance` _tolerance_5) (== _relativelocation_5 (`SceneComponent.RelativeLocation` (`self.Orbiter4`)) :`ErrorTolerance` _tolerance_5) (== _relativelocation_5 (`SceneComponent.RelativeLocation` (`self.Orbiter9`)) :`ErrorTolerance` _tolerance_5) (== _relativelocation_5 (`SceneComponent.RelativeLocation` (`self.Orbiter10`)) :`ErrorTolerance` _tolerance_5) (== _relativelocation_5 (`SceneComponent.RelativeLocation` (`self.Orbiter11`)) :`ErrorTolerance` _tolerance_5)) (or (== _relativelocation_6 (`SceneComponent.RelativeLocation` (`self.Orbiter0`)) :`ErrorTolerance` _tolerance_6) (== _relativelocation_6 (`SceneComponent.RelativeLocation` (`self.Orbiter2`)) :`ErrorTolerance` _tolerance_6) (== _relativelocation_6 (`SceneComponent.RelativeLocation` (`self.Orbiter4`)) :`ErrorTolerance` _tolerance_6) (== _relativelocation_6 (`SceneComponent.RelativeLocation` (`self.Orbiter9`)) :`ErrorTolerance` _tolerance_6) (== _relativelocation_6 (`SceneComponent.RelativeLocation` (`self.Orbiter10`)) :`ErrorTolerance` _tolerance_6) (== _relativelocation_6 (`SceneComponent.RelativeLocation` (`self.Orbiter11`)) :`ErrorTolerance` _tolerance_6)) (or (== _relativelocation (`SceneComponent.RelativeLocation` (`self.Orbiter0`)) :`ErrorTolerance` _tolerance) (== _relativelocation (`SceneComponent.RelativeLocation` (`self.Orbiter2`)) :`ErrorTolerance` _tolerance) (== _relativelocation (`SceneComponent.RelativeLocation` (`self.Orbiter4`)) :`ErrorTolerance` _tolerance) (== _relativelocation (`SceneComponent.RelativeLocation` (`self.Orbiter9`)) :`ErrorTolerance` _tolerance) (== _relativelocation (`SceneComponent.RelativeLocation` (`self.Orbiter10`)) :`ErrorTolerance` _tolerance) (== _relativelocation (`SceneComponent.RelativeLocation` (`self.Orbiter11`)) :`ErrorTolerance` _tolerance)))
          (`MeshComponent.SetVectorParameterValueOnMaterials` (`self.Torus2`) "Color" (0.0 2.2 1.0))
          (`MeshComponent.SetVectorParameterValueOnMaterials` (`self.Torus1`) "Color" (0.0 2.2 1.0))
          (`MeshComponent.SetVectorParameterValueOnMaterials` (`self.ButtonUp`) "Color" (0.0 2.2 1.0))
          (`MeshComponent.SetVectorParameterValueOnMaterials` (`self.ButtonRight`) "Color" (0.0 2.2 1.0))
          (`MeshComponent.SetVectorParameterValueOnMaterials` (`self.ButtonLeft`) "Color" (0.0 2.2 1.0))
          (`MeshComponent.SetVectorParameterValueOnMaterials` (`self.Torus3`) "Color" (0.0 2.2 1.0))
          (`MeshComponent.SetVectorParameterValueOnMaterials` (`self.Orbiter0`) "Color" (0.0 2.2 1.0))
          (`MeshComponent.SetVectorParameterValueOnMaterials` (`self.Orbiter2`) "Color" (0.0 2.2 1.0))
          (`MeshComponent.SetVectorParameterValueOnMaterials` (`self.Orbiter4`) "Color" (0.0 2.2 1.0))
          (`MeshComponent.SetVectorParameterValueOnMaterials` (`self.Orbiter9`) "Color" (0.0 2.2 1.0))
          (`MeshComponent.SetVectorParameterValueOnMaterials` (`self.Orbiter10`) "Color" (0.0 2.2 1.0))
          (`MeshComponent.SetVectorParameterValueOnMaterials` (`self.Orbiter11`) "Color" (0.0 2.2 1.0))
          (`MeshComponent.SetVectorParameterValueOnMaterials` (`self.Torus4`) "Color" (0.0 2.2 1.0))
          (`MeshComponent.SetVectorParameterValueOnMaterials` (`self.Torus5`) "Color" (0.0 2.2 1.0))
          (`MeshComponent.SetVectorParameterValueOnMaterials` (`self.Torus6`) "Color" (0.0 2.2 1.0))
          (`MeshComponent.SetScalarParameterValueOnMaterials` (`self.Torus3`) "Intensity" 8.0)
          (`MeshComponent.SetScalarParameterValueOnMaterials` (`self.Torus2`) "Intensity" 8.0)
          (`MeshComponent.SetScalarParameterValueOnMaterials` (`self.Torus1`) "Intensity" 8.0)
          (`MeshComponent.SetScalarParameterValueOnMaterials` (`self.ButtonUp`) "Intensity" 8.0)
          (`MeshComponent.SetScalarParameterValueOnMaterials` (`self.ButtonRight`) "Intensity" 8.0)
          (`MeshComponent.SetScalarParameterValueOnMaterials` (`self.ButtonLeft`) "Intensity" 8.0)
          (`MeshComponent.SetScalarParameterValueOnMaterials` (`self.Orbiter0`) "Intensity" 8.0)
          (`MeshComponent.SetScalarParameterValueOnMaterials` (`self.Orbiter2`) "Intensity" 8.0)
          (`MeshComponent.SetScalarParameterValueOnMaterials` (`self.Orbiter4`) "Intensity" 8.0)
          (`MeshComponent.SetScalarParameterValueOnMaterials` (`self.Orbiter9`) "Intensity" 8.0)
          (`MeshComponent.SetScalarParameterValueOnMaterials` (`self.Orbiter10`) "Intensity" 8.0)
          (`MeshComponent.SetScalarParameterValueOnMaterials` (`self.Orbiter11`) "Intensity" 8.0)
          (`MeshComponent.SetScalarParameterValueOnMaterials` (`self.Torus4`) "Intensity" 8.0)
          (`MeshComponent.SetScalarParameterValueOnMaterials` (`self.Torus5`) "Intensity" 8.0)
          (`MeshComponent.SetScalarParameterValueOnMaterials` (`self.Torus6`) "Intensity" 8.0)
          (`MeshComponent.SetScalarParameterValueOnMaterials` (`self.Orbiter1`) "Intensity" 10.0)
          (`MeshComponent.SetScalarParameterValueOnMaterials` (`self.Orbiter3`) "Intensity" 10.0)
          (`MeshComponent.SetScalarParameterValueOnMaterials` (`self.Orbiter5`) "Intensity" 10.0)
          (`MeshComponent.SetScalarParameterValueOnMaterials` (`self.Orbiter6`) "Intensity" 10.0)
          (`MeshComponent.SetScalarParameterValueOnMaterials` (`self.Orbiter7`) "Intensity" 10.0)
          (`MeshComponent.SetScalarParameterValueOnMaterials` (`self.Orbiter8`) "Intensity" 10.0))))
    (else
      (goto _label))))

(event `self.ReceiveActorOnClicked`
  (params (ButtonPressed :type "Key Structure"))
  (bind _buttonup (`self.ButtonUp`))
  (bind _buttonright (`self.ButtonRight`))
  (bind _buttonleft (`self.ButtonLeft`))
  (bind _hitresult (`PlayerController.GetHitResultUnderCursorForObjects` (`GameplayStatics.GetPlayerController` 0) (`|MakeArray` "ObjectTypeQuery7" :!type "EObjectTypeQuery Enum") true))
  ;[1 1 1] Turn Around Orbit
  (if (`GameplayStatics.BreakHitResult` _hitresult)
    (for _array_element (`self.Pieces`)
      (if (== _array_element (`.HitComponent` (`GameplayStatics.BreakHitResult` _hitresult)))
        (`|ExecutionSequence`
          (:`then_0`
            (if (== (`.HitComponent` (`GameplayStatics.BreakHitResult` _hitresult)) _buttonup)
              (set `self.OrbitCenter` (`SceneComponent.RelativeLocation` _buttonup))))
          (:`then_1`
            (if (== (`.HitComponent` (`GameplayStatics.BreakHitResult` _hitresult)) _buttonright)
              (set `self.OrbitCenter` (`SceneComponent.RelativeLocation` _buttonright))))
          (:`then_2`
            (if (== (`.HitComponent` (`GameplayStatics.BreakHitResult` _hitresult)) _buttonleft)
              (set `self.OrbitCenter` (`SceneComponent.RelativeLocation` _buttonleft))))
          (:`then_3`
            (for _array_element_2 (`SceneComponent.GetChildrenComponents` (`self.Orbiter`) false)
              (bind (_relativelocation_x _relativelocation_y) (`KismetMathLibrary.BreakVector` (`SceneComponent.RelativeLocation` _array_element_2)))
              (if (and (<= (`KismetMathLibrary.Distance2D` (`KismetMathLibrary.Conv_VectorToVector2D` (`self.OrbitCenter`)) (`KismetMathLibrary.MakeVector2D` _relativelocation_x _relativelocation_y)) (+ (`self.Radius`) 10.0)) (!= (`self.ButtonRight`) _array_element_2) (!= (`self.ButtonLeft`) _array_element_2) (!= (`self.ButtonUp`) _array_element_2))
                (bind _returnvalue (- (`SceneComponent.RelativeLocation` _array_element_2) (`self.OrbitCenter`)))
                (`SceneComponent.K2_AddLocalOffset` _array_element_2 (- (`KismetMathLibrary.RotateAngleAxis` _returnvalue 60.0 (0.0 0.0 1.0)) _returnvalue) false false)))))))))

(fn `UserConstructionScript`
  (locals (Blue :type "Color Structure" :default (struct :`B` 255 :`G` 129)) (Green :type "Color Structure" :default (struct :`G` 255)) (OrbiterZ :type "Float (double-precision)" :default 0.0))
  (bind _radius (`self.Radius`))
  (bind _orbiterz (`local.OrbiterZ`))
  (bind (_relativelocation_x _relativelocation_y) (`KismetMathLibrary.BreakVector` (`SceneComponent.RelativeLocation` (`self.Orbiter2`))))
  (bind (_relativelocation_x_2 _relativelocation_y_2) (`KismetMathLibrary.BreakVector` (`SceneComponent.RelativeLocation` (`self.Orbiter2`))))
  (bind (_relativelocation_x_3 _relativelocation_y_3) (`KismetMathLibrary.BreakVector` (`SceneComponent.RelativeLocation` (`self.Orbiter2`))))
  (bind (_relativelocation_x_4 _relativelocation_y_4) (`KismetMathLibrary.BreakVector` (`SceneComponent.RelativeLocation` (`self.Orbiter2`))))
  (bind (_relativelocation_x_5 _relativelocation_y_5) (`KismetMathLibrary.BreakVector` (`SceneComponent.RelativeLocation` (`self.Orbiter1`))))
  (bind (_relativelocation_x_6 _relativelocation_y_6) (`KismetMathLibrary.BreakVector` (`SceneComponent.RelativeLocation` (`self.Orbiter1`))))
  (bind _returnvalue (`KismetMathLibrary.Conv_LinearColorToVector` (`KismetMathLibrary.Conv_ColorToLinearColor` (`local.Green`))))
  (`|ExecutionSequence`
    (:`then_0`
      ;[1 1 1] Add buttons in Pieces array
      (`KismetArrayLibrary.Array_Add` (`self.Pieces`) (`self.ButtonRight`))
      (`KismetArrayLibrary.Array_Add` (`self.Pieces`) (`self.ButtonUp`))
      (`KismetArrayLibrary.Array_Add` (`self.Pieces`) (`self.ButtonLeft`)))
    (:`then_1`
      ;[1 1 1] Set Pieces Intensity And Color
      (`MeshComponent.SetVectorParameterValueOnMaterials` (`self.Torus1`) "Color" (0.0 1.0 0.0))
      (`MeshComponent.SetVectorParameterValueOnMaterials` (`self.Torus3`) "Color" (0.0 1.0 0.0))
      (`MeshComponent.SetVectorParameterValueOnMaterials` (`self.Torus2`) "Color" (0.0 1.0 0.0))
      (`MeshComponent.SetVectorParameterValueOnMaterials` (`self.ButtonLeft`) "Color" (0.0 1.0 0.0))
      (`MeshComponent.SetVectorParameterValueOnMaterials` (`self.ButtonUp`) "Color" (0.0 1.0 0.0))
      (`MeshComponent.SetVectorParameterValueOnMaterials` (`self.ButtonRight`) "Color" (0.0 1.0 0.0))
      (`MeshComponent.SetVectorParameterValueOnMaterials` (`self.Torus4`) "Color" (0.0 1.0 0.0))
      (`MeshComponent.SetVectorParameterValueOnMaterials` (`self.Torus5`) "Color" (0.0 1.0 0.0))
      (`MeshComponent.SetVectorParameterValueOnMaterials` (`self.Torus6`) "Color" (0.0 1.0 0.0))
      (`MeshComponent.SetVectorParameterValueOnMaterials` (`self.Torus7`) "Color" (1.0 0.0 0.0))
      (`MeshComponent.SetVectorParameterValueOnMaterials` (`self.Torus8`) "Color" (1.0 0.0 0.0))
      (`MeshComponent.SetVectorParameterValueOnMaterials` (`self.Torus9`) "Color" (1.0 0.0 0.0))
      (`MeshComponent.SetVectorParameterValueOnMaterials` (`self.Torus10`) "Color" (1.0 0.0 0.0))
      (`MeshComponent.SetVectorParameterValueOnMaterials` (`self.Torus11`) "Color" (1.0 0.0 0.0))
      (`MeshComponent.SetVectorParameterValueOnMaterials` (`self.Torus12`) "Color" (1.0 0.0 0.0))
      (`MeshComponent.SetScalarParameterValueOnMaterials` (`self.Torus11`) "Intensity" 3.0)
      (`MeshComponent.SetScalarParameterValueOnMaterials` (`self.Torus10`) "Intensity" 3.0)
      (`MeshComponent.SetScalarParameterValueOnMaterials` (`self.Torus9`) "Intensity" 3.0)
      (`MeshComponent.SetScalarParameterValueOnMaterials` (`self.Torus7`) "Intensity" 3.0)
      (`MeshComponent.SetScalarParameterValueOnMaterials` (`self.Torus8`) "Intensity" 3.0)
      (`MeshComponent.SetScalarParameterValueOnMaterials` (`self.Torus1`) "Intensity" 3.0)
      (`MeshComponent.SetScalarParameterValueOnMaterials` (`self.Torus2`) "Intensity" 3.0)
      (`MeshComponent.SetScalarParameterValueOnMaterials` (`self.Torus3`) "Intensity" 3.0)
      (`MeshComponent.SetScalarParameterValueOnMaterials` (`self.Torus12`) "Intensity" 3.0)
      (`MeshComponent.SetScalarParameterValueOnMaterials` (`self.ButtonRight`) "Intensity" 3.0)
      (`MeshComponent.SetScalarParameterValueOnMaterials` (`self.ButtonUp`) "Intensity" 3.0)
      (`MeshComponent.SetScalarParameterValueOnMaterials` (`self.ButtonLeft`) "Intensity" 3.0)
      (`MeshComponent.SetScalarParameterValueOnMaterials` (`self.Torus4`) "Intensity" 3.0)
      (`MeshComponent.SetScalarParameterValueOnMaterials` (`self.Torus5`) "Intensity" 3.0)
      (`MeshComponent.SetScalarParameterValueOnMaterials` (`self.Torus6`) "Intensity" 3.0)
      (`MeshComponent.SetVectorParameterValueOnMaterials` (`self.Orbiter1`) "Color" (1.0 0.0 0.0))
      (`MeshComponent.SetVectorParameterValueOnMaterials` (`self.Orbiter3`) "Color" (1.0 0.0 0.0))
      (`MeshComponent.SetVectorParameterValueOnMaterials` (`self.Orbiter5`) "Color" (1.0 0.0 0.0))
      (`MeshComponent.SetVectorParameterValueOnMaterials` (`self.Orbiter6`) "Color" (1.0 0.0 0.0))
      (`MeshComponent.SetVectorParameterValueOnMaterials` (`self.Orbiter8`) "Color" (1.0 0.0 0.0))
      (`MeshComponent.SetVectorParameterValueOnMaterials` (`self.Orbiter7`) "Color" (1.0 0.0 0.0))
      (`MeshComponent.SetVectorParameterValueOnMaterials` (`self.Orbiter2`) "Color" _returnvalue)
      (`MeshComponent.SetVectorParameterValueOnMaterials` (`self.Orbiter4`) "Color" _returnvalue)
      (`MeshComponent.SetVectorParameterValueOnMaterials` (`self.Orbiter9`) "Color" _returnvalue)
      (`MeshComponent.SetVectorParameterValueOnMaterials` (`self.Orbiter0`) "Color" _returnvalue)
      (`MeshComponent.SetVectorParameterValueOnMaterials` (`self.Orbiter10`) "Color" _returnvalue)
      (`MeshComponent.SetVectorParameterValueOnMaterials` (`self.Orbiter11`) "Color" _returnvalue)
      (`MeshComponent.SetScalarParameterValueOnMaterials` (`self.Orbiter0`) "Intensity" 5.0)
      (`MeshComponent.SetScalarParameterValueOnMaterials` (`self.Orbiter2`) "Intensity" 5.0)
      (`MeshComponent.SetScalarParameterValueOnMaterials` (`self.Orbiter4`) "Intensity" 5.0)
      (`MeshComponent.SetScalarParameterValueOnMaterials` (`self.Orbiter11`) "Intensity" 5.0)
      (`MeshComponent.SetScalarParameterValueOnMaterials` (`self.Orbiter10`) "Intensity" 5.0)
      (`MeshComponent.SetScalarParameterValueOnMaterials` (`self.Orbiter9`) "Intensity" 5.0)
      (`MeshComponent.SetScalarParameterValueOnMaterials` (`self.Orbiter3`) "Intensity" 8.0)
      (`MeshComponent.SetScalarParameterValueOnMaterials` (`self.Orbiter6`) "Intensity" 8.0)
      (`MeshComponent.SetScalarParameterValueOnMaterials` (`self.Orbiter5`) "Intensity" 8.0)
      (`MeshComponent.SetScalarParameterValueOnMaterials` (`self.Orbiter8`) "Intensity" 8.0)
      (`MeshComponent.SetScalarParameterValueOnMaterials` (`self.Orbiter1`) "Intensity" 8.0)
      (`MeshComponent.SetScalarParameterValueOnMaterials` (`self.Orbiter7`) "Intensity" 8.0)
      ;[1 1 1] Set Orbital Positions
      (`SceneComponent.K2_SetRelativeLocation` (`self.Orbiter1`) (`KismetMathLibrary.MakeVector` (* (`KismetMathLibrary.DegCos` 60.0) _radius) (* (`KismetMathLibrary.DegSin` 60.0) _radius) _orbiterz) false false)
      (`SceneComponent.K2_SetRelativeLocation` (`self.ButtonRight`) (`KismetMathLibrary.MakeVector` (* (`KismetMathLibrary.DegCos` 60.0) _radius) (* (`KismetMathLibrary.DegSin` 60.0) _radius) _orbiterz) false false)
      (`SceneComponent.K2_SetRelativeLocation` (`self.Torus4`) (`KismetMathLibrary.MakeVector` (* (`KismetMathLibrary.DegCos` 60.0) _radius) (* (`KismetMathLibrary.DegSin` 60.0) _radius) _orbiterz) false false)
      (`SceneComponent.K2_SetRelativeLocation` (`self.Orbiter2`) (`KismetMathLibrary.MakeVector` (* (`KismetMathLibrary.DegCos` 120.0) _radius) (* (`KismetMathLibrary.DegSin` 120.0) _radius) _orbiterz) false false)
      (`SceneComponent.K2_SetRelativeLocation` (`self.ButtonLeft`) (`KismetMathLibrary.MakeVector` (* (`KismetMathLibrary.DegCos` 120.0) _radius) (* (`KismetMathLibrary.DegSin` 120.0) _radius) _orbiterz) false false)
      (`SceneComponent.K2_SetRelativeLocation` (`self.Torus5`) (`KismetMathLibrary.MakeVector` (* (`KismetMathLibrary.DegCos` 120.0) _radius) (* (`KismetMathLibrary.DegSin` 120.0) _radius) _orbiterz) false false)
      (`SceneComponent.K2_SetRelativeLocation` (`self.Orbiter3`) (`KismetMathLibrary.MakeVector` (* (`KismetMathLibrary.DegCos` 180.0) _radius) (* (`KismetMathLibrary.DegSin` 180.0) _radius) _orbiterz) false false)
      (`SceneComponent.K2_SetRelativeLocation` (`self.Torus2`) (`KismetMathLibrary.MakeVector` (* (`KismetMathLibrary.DegCos` 180.0) _radius) (* (`KismetMathLibrary.DegSin` 180.0) _radius) _orbiterz) false false)
      (`SceneComponent.K2_SetRelativeLocation` (`self.Orbiter4`) (`KismetMathLibrary.MakeVector` (* (`KismetMathLibrary.DegCos` 240.0) _radius) (* (`KismetMathLibrary.DegSin` 240.0) _radius) _orbiterz) false false)
      (`SceneComponent.K2_SetRelativeLocation` (`self.Torus7`) (`KismetMathLibrary.MakeVector` (* (`KismetMathLibrary.DegCos` 240.0) _radius) (* (`KismetMathLibrary.DegSin` 240.0) _radius) _orbiterz) false false)
      (`SceneComponent.K2_SetRelativeLocation` (`self.Orbiter5`) (`KismetMathLibrary.MakeVector` (* (`KismetMathLibrary.DegCos` 300.0) _radius) (* (`KismetMathLibrary.DegSin` 300.0) _radius) _orbiterz) false false)
      (`SceneComponent.K2_SetRelativeLocation` (`self.Torus8`) (`KismetMathLibrary.MakeVector` (* (`KismetMathLibrary.DegCos` 300.0) _radius) (* (`KismetMathLibrary.DegSin` 300.0) _radius) _orbiterz) false false)
      (`SceneComponent.K2_SetRelativeLocation` (`self.Orbiter6`) (`KismetMathLibrary.MakeVector` (* (`KismetMathLibrary.DegCos` 360.0) _radius) (* (`KismetMathLibrary.DegSin` 360.0) _radius) _orbiterz) false false)
      (`SceneComponent.K2_SetRelativeLocation` (`self.Torus3`) (`KismetMathLibrary.MakeVector` (* (`KismetMathLibrary.DegCos` 360.0) _radius) (* (`KismetMathLibrary.DegSin` 360.0) _radius) _orbiterz) false false)
      (`SceneComponent.K2_SetRelativeLocation` (`self.Orbiter0`) (`KismetMathLibrary.MakeVector` (+ _relativelocation_x (* (`KismetMathLibrary.DegCos` 60.0) _radius)) (+ _relativelocation_y (* (`KismetMathLibrary.DegSin` 60.0) _radius)) _orbiterz) false false)
      (`SceneComponent.K2_SetRelativeLocation` (`self.Torus1`) (`KismetMathLibrary.MakeVector` (+ _relativelocation_x (* (`KismetMathLibrary.DegCos` 60.0) _radius)) (+ _relativelocation_y (* (`KismetMathLibrary.DegSin` 60.0) _radius)) _orbiterz) false false)
      (`SceneComponent.K2_SetRelativeLocation` (`self.Orbiter7`) (`KismetMathLibrary.MakeVector` (+ _relativelocation_x_2 (* (`KismetMathLibrary.DegCos` 120.0) _radius)) (+ _relativelocation_y_2 (* (`KismetMathLibrary.DegSin` 120.0) _radius)) _orbiterz) false false)
      (`SceneComponent.K2_SetRelativeLocation` (`self.Torus12`) (`KismetMathLibrary.MakeVector` (+ _relativelocation_x_2 (* (`KismetMathLibrary.DegCos` 120.0) _radius)) (+ _relativelocation_y_2 (* (`KismetMathLibrary.DegSin` 120.0) _radius)) _orbiterz) false false)
      (`SceneComponent.K2_SetRelativeLocation` (`self.Orbiter8`) (`KismetMathLibrary.MakeVector` (+ _relativelocation_x_3 (* (`KismetMathLibrary.DegCos` 180.0) _radius)) (+ _relativelocation_y_3 (* (`KismetMathLibrary.DegSin` 180.0) _radius)) _orbiterz) false false)
      (`SceneComponent.K2_SetRelativeLocation` (`self.Torus9`) (`KismetMathLibrary.MakeVector` (+ _relativelocation_x_3 (* (`KismetMathLibrary.DegCos` 180.0) _radius)) (+ _relativelocation_y_3 (* (`KismetMathLibrary.DegSin` 180.0) _radius)) _orbiterz) false false)
      (`SceneComponent.K2_SetRelativeLocation` (`self.Orbiter9`) (`KismetMathLibrary.MakeVector` (+ _relativelocation_x_4 (* (`KismetMathLibrary.DegCos` 300.0) _radius)) (+ _relativelocation_y_4 (* (`KismetMathLibrary.DegSin` 300.0) _radius)) _orbiterz) false false)
      (`SceneComponent.K2_SetRelativeLocation` (`self.ButtonUp`) (`KismetMathLibrary.MakeVector` (+ _relativelocation_x_4 (* (`KismetMathLibrary.DegCos` 300.0) _radius)) (+ _relativelocation_y_4 (* (`KismetMathLibrary.DegSin` 300.0) _radius)) _orbiterz) false false)
      (`SceneComponent.K2_SetRelativeLocation` (`self.Orbiter10`) (`KismetMathLibrary.MakeVector` (+ _relativelocation_x_5 (* (`KismetMathLibrary.DegCos` 0.0) _radius)) (+ _relativelocation_y_5 (* (`KismetMathLibrary.DegSin` 0.0) _radius)) _orbiterz) false false)
      (`SceneComponent.K2_SetRelativeLocation` (`self.Torus11`) (`KismetMathLibrary.MakeVector` (+ _relativelocation_x_5 (* (`KismetMathLibrary.DegCos` 0.0) _radius)) (+ _relativelocation_y_5 (* (`KismetMathLibrary.DegSin` 0.0) _radius)) _orbiterz) false false)
      (`SceneComponent.K2_SetRelativeLocation` (`self.Orbiter11`) (`KismetMathLibrary.MakeVector` (+ _relativelocation_x_6 (* (`KismetMathLibrary.DegCos` 60.0) _radius)) (+ _relativelocation_y_6 (* (`KismetMathLibrary.DegSin` 60.0) _radius)) _orbiterz) false false)
      (`SceneComponent.K2_SetRelativeLocation` (`self.Torus10`) (`KismetMathLibrary.MakeVector` (+ _relativelocation_x_6 (* (`KismetMathLibrary.DegCos` 60.0) _radius)) (+ _relativelocation_y_6 (* (`KismetMathLibrary.DegSin` 60.0) _radius)) _orbiterz) false false))
    (:`then_2`
      ;[1 1 1] Set Camera Position
      (`SceneComponent.K2_SetRelativeTransform` (`self.Camera`) (`self.CameraTransform`) false false))))