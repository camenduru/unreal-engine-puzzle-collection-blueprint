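; BP_RotatingPuzzle is a puzzle actor where the player clicks four pieces (Canvas, Out, Middle, In) to rotate them 90 degrees toward zero rotation.
; ActivateCamera blends to the puzzle view, enables mouse interaction and starts a frame-delta looping timer, which DeactivateCamera clears.
; The timer highlights hovered pieces through custom depth and polls rotations, switching material colour and intensity when all align.
; The construction script sets piece materials and camera transform.
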(event `/Game/CPCP1/Utilities/Character/Blueprints/BP_PuzzleInterface.DeactivateCamera`
  ;[1 1 1] Exit Puzzle
  (`KismetSystemLibrary.K2_ClearAndInvalidateTimerHandle` (`self.TimerHandle`))
  (for _array_element (`self.Pieces`)
    (`PrimitiveComponent.SetRenderCustomDepth` _array_element false)))

(event `/Game/CPCP1/Utilities/Character/Blueprints/BP_PuzzleInterface.ActivateCamera`
  (bind _returnvalue (`GameplayStatics.GetPlayerController` 0))
  (bind (_returnvalue_x _returnvalue_y) (`KismetMathLibrary.BreakVector2D` (`WidgetLayoutLibrary.GetViewportSize`)))
  (bind _returnvalue_2 (`GameplayStatics.GetPlayerController` 0))
  (bind _returnvalue_3 (`GameplayStatics.GetPlayerController` 0))
  ;[1 1 1] Enter To Puzzle
  (`PlayerController.SetMouseLocation` _returnvalue_2 (`KismetMathLibrary.FTrunc` (/ _returnvalue_x 2.0)) (`KismetMathLibrary.FTrunc` (/ _returnvalue_y 2.0)))
  (`WidgetBlueprintLibrary.SetInputMode_GameAndUIEx` _returnvalue_2 null "DoNotLock" false)
  (`Controller.SetIgnoreLookInput` _returnvalue_3 true)
  (`Controller.SetIgnoreMoveInput` _returnvalue_3 true)
  (`PlayerController.SetViewTargetWithBlend` _returnvalue_3 self 0.5 "VTBlend_Linear" 0.0 false)
  (set `PlayerController.bEnableClickEvents` true _returnvalue)
  (set `PlayerController.bEnableMouseOverEvents` true _returnvalue)
  (set `PlayerController.bShowMouseCursor` true _returnvalue)
  (`WidgetLayoutLibrary.RemoveAllWidgets`)
  ;[1 1 1] Drag And Drop
  (bind _returnvalue_4 (`KismetSystemLibrary.K2_SetTimerDelegate` (delegate `TimerEvent`) (`GameplayStatics.GetWorldDeltaSeconds`) true))
  (set `self.TimerHandle` _returnvalue_4))

(event `TimerEvent`
  (bind _returnvalue (`GameplayStatics.GetPlayerController` 0))
  (bind _winintensity (`self.WinIntensity`))
  (bind _out (`self.Out`))
  (bind _middle (`self.Middle`))
  (bind _in (`self.In`))
  (bind _canvas (`self.Canvas`))
  (bind _hitresult (`PlayerController.GetHitResultUnderCursorForObjects` (`GameplayStatics.GetPlayerController` 0) (`|MakeArray` "ObjectTypeQuery7" :!type "EObjectTypeQuery Enum") true))
  (bind _returnvalue_2 (`KismetMathLibrary.Conv_LinearColorToVector` (`KismetMathLibrary.Conv_ColorToLinearColor` (`self.WinColor`))))
  ;[1 1 1] Check Is Puzzle Active
  (bind _asbp_puzzle_character (cast `/Game/CPCP1/Utilities/Character/Blueprints/BP_PuzzleCharacter` (`GameplayStatics.GetPlayerCharacter` 0)))
  (if (`/Game/CPCP1/Utilities/Character/Blueprints/BP_PuzzleCharacter.isPuzzleActive` _asbp_puzzle_character)
    (`|ExecutionSequence`
      (:`then_0`
        ;[1 1 1] Drag And Drop
        (if (`GameplayStatics.BreakHitResult` _hitresult)
          (for _array_element (`self.Pieces`)
            (if (== _array_element (`.HitComponent` (`GameplayStatics.BreakHitResult` _hitresult)))
              (`PrimitiveComponent.SetRenderCustomDepth` _array_element true)
              (set `PlayerController.CurrentMouseCursor` "GrabHand" _returnvalue)
              (for _array_element_2 (`self.Pieces`)
                (if (!= _array_element_2 _array_element)
                  (`PrimitiveComponent.SetRenderCustomDepth` _array_element_2 false)))))
          (else
            (for _array_element_3 (`self.Pieces`) :!label _label
              (`PrimitiveComponent.SetRenderCustomDepth` _array_element_3 false)
              (set `PlayerController.CurrentMouseCursor` "Default" _returnvalue)))))
      (:`then_1`
        ;[1 1 1] WinCondition
        (if (and (== (`SceneComponent.RelativeRotation` _canvas) (struct)) (== (`SceneComponent.RelativeRotation` _out) (struct)) (== (`SceneComponent.RelativeRotation` _middle) (struct)) (== (`SceneComponent.RelativeRotation` _in) (struct)))
          (`|ExecutionSequence`
            (:`then_0`
              (`MeshComponent.SetVectorParameterValueOnMaterials` _canvas "Color" _returnvalue_2)
              (`MeshComponent.SetScalarParameterValueOnMaterials` _canvas "Intensity" _winintensity))
            (:`then_1`
              (`MeshComponent.SetVectorParameterValueOnMaterials` _out "Color" _returnvalue_2)
              (`MeshComponent.SetScalarParameterValueOnMaterials` _out "Intensity" _winintensity))
            (:`then_2`
              (`MeshComponent.SetVectorParameterValueOnMaterials` _middle "Color" _returnvalue_2)
              (`MeshComponent.SetScalarParameterValueOnMaterials` _middle "Intensity" _winintensity))
            (:`then_3`
              (`MeshComponent.SetVectorParameterValueOnMaterials` _in "Color" _returnvalue_2)
              (`MeshComponent.SetScalarParameterValueOnMaterials` _in "Intensity" _winintensity)))
          (else
            (`|ExecutionSequence`
              (:`then_0`
                (`MeshComponent.SetVectorParameterValueOnMaterials` _canvas "Color" (`KismetMathLibrary.Conv_LinearColorToVector` (`KismetMathLibrary.Conv_ColorToLinearColor` (`self.CanvasColor`))))
                (`MeshComponent.SetScalarParameterValueOnMaterials` _canvas "Intensity" 1.0))
              (:`then_1`
                (`MeshComponent.SetVectorParameterValueOnMaterials` _out "Color" (`KismetMathLibrary.Conv_LinearColorToVector` (`KismetMathLibrary.Conv_ColorToLinearColor` (`self.OutColor`))))
                (`MeshComponent.SetScalarParameterValueOnMaterials` _out "Intensity" 1.0))
              (:`then_2`
                (`MeshComponent.SetVectorParameterValueOnMaterials` _middle "Color" (`KismetMathLibrary.Conv_LinearColorToVector` (`KismetMathLibrary.Conv_ColorToLinearColor` (`self.MiddleColor`))))
                (`MeshComponent.SetScalarParameterValueOnMaterials` _middle "Intensity" 1.0))
              (:`then_3`
                (`MeshComponent.SetVectorParameterValueOnMaterials` _in "Color" (`KismetMathLibrary.Conv_LinearColorToVector` (`KismetMathLibrary.Conv_ColorToLinearColor` (`self.InColor`))))
                (`MeshComponent.SetScalarParameterValueOnMaterials` _in "Intensity" 1.0)))))))
    (else
      (goto _label))))

(event `self.ReceiveActorOnClicked`
  (params (ButtonPressed :type "Key Structure"))
  (bind _hitresult (`PlayerController.GetHitResultUnderCursorForObjects` (`GameplayStatics.GetPlayerController` 0) (`|MakeArray` "ObjectTypeQuery7" :!type "EObjectTypeQuery Enum") true))
  ;[1 1 1] Click
  (bind _asbp_puzzle_character (cast `/Game/CPCP1/Utilities/Character/Blueprints/BP_PuzzleCharacter` (`GameplayStatics.GetPlayerCharacter` 0)))
  (if (`/Game/CPCP1/Utilities/Character/Blueprints/BP_PuzzleCharacter.isPuzzleActive` _asbp_puzzle_character)
    (if (`GameplayStatics.BreakHitResult` _hitresult)
      (for _array_element (`self.Pieces`)
        (if (== _array_element (`.HitComponent` (`GameplayStatics.BreakHitResult` _hitresult)))
          (`SceneComponent.K2_AddRelativeRotation` _array_element (struct :`Roll` 90.0) false false))))))

(fn `UserConstructionScript`
  (bind _middle (`self.Middle`))
  (bind _uvtiling (`self.UVTiling`))
  (bind _uvtiling_2 (`self.UVTiling`))
  (bind _uvtiling_3 (`self.UVTiling`))
  (bind _out (`self.Out`))
  (bind _uvtiling_4 (`self.UVTiling`))
  (bind _in (`self.In`))
  (bind _random (`self.Random`))
  (bind _canvas (`self.Canvas`))
  (`|ExecutionSequence`
    (:`then_0`
      ;[1 1 1] Add In Pieces Array
      (`KismetArrayLibrary.Array_Add` (`self.Pieces`) (`self.Out`))
      (`KismetArrayLibrary.Array_Add` (`self.Pieces`) (`self.Middle`))
      (`KismetArrayLibrary.Array_Add` (`self.Pieces`) (`self.In`))
      (`KismetArrayLibrary.Array_Add` (`self.Pieces`) (`self.Canvas`)))
    (:`then_1`
      ;[1 1 1] Set Intensity Color And Tiling For Each Piece
      (`MeshComponent.SetScalarParameterValueOnMaterials` _in "Random" _random)
      (`MeshComponent.SetVectorParameterValueOnMaterials` _in "Color" (`KismetMathLibrary.Conv_LinearColorToVector` (`KismetMathLibrary.Conv_ColorToLinearColor` (`self.InColor`))))
      (`MeshComponent.SetScalarParameterValueOnMaterials` _in "Intensity" (`self.InIntensity`))
      (`MeshComponent.SetScalarParameterValueOnMaterials` _in "UTiling" _uvtiling_4)
      (`MeshComponent.SetScalarParameterValueOnMaterials` _in "VTiling" _uvtiling_4)
      (`MeshComponent.SetVectorParameterValueOnMaterials` _middle "Color" (`KismetMathLibrary.Conv_LinearColorToVector` (`KismetMathLibrary.Conv_ColorToLinearColor` (`self.MiddleColor`))))
      (`MeshComponent.SetScalarParameterValueOnMaterials` _middle "Random" _random)
      (`MeshComponent.SetScalarParameterValueOnMaterials` _middle "Intensity" (`self.MiddleIntensity`))
      (`MeshComponent.SetScalarParameterValueOnMaterials` _middle "UTiling" _uvtiling_3)
      (`MeshComponent.SetScalarParameterValueOnMaterials` _middle "VTiling" _uvtiling_3)
      (`MeshComponent.SetScalarParameterValueOnMaterials` _out "Random" _random)
      (`MeshComponent.SetVectorParameterValueOnMaterials` _out "Color" (`KismetMathLibrary.Conv_LinearColorToVector` (`KismetMathLibrary.Conv_ColorToLinearColor` (`self.OutColor`))))
      (`MeshComponent.SetScalarParameterValueOnMaterials` _out "Intensity" (`self.OutIntensity`))
      (`MeshComponent.SetScalarParameterValueOnMaterials` _out "UTiling" _uvtiling)
      (`MeshComponent.SetScalarParameterValueOnMaterials` _out "VTiling" _uvtiling)
      (`MeshComponent.SetScalarParameterValueOnMaterials` _canvas "Random" _random)
      (`MeshComponent.SetScalarParameterValueOnMaterials` _canvas "Intensity" (`self.CanvasIntensity`))
      (`MeshComponent.SetScalarParameterValueOnMaterials` _canvas "UTiling" _uvtiling_2)
      (`MeshComponent.SetScalarParameterValueOnMaterials` _canvas "VTiling" _uvtiling_2)
      (`MeshComponent.SetVectorParameterValueOnMaterials` _canvas "Color" (`KismetMathLibrary.Conv_LinearColorToVector` (`KismetMathLibrary.Conv_ColorToLinearColor` (`self.CanvasColor`)))))
    (:`then_2`
      ;[1 1 1] Set Camera Position
      (`SceneComponent.K2_SetRelativeTransform` (`self.Camera`) (`self.CameraTransform`) false false))))